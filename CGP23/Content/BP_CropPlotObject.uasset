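; BP_CropPlotObject is a crop plot that holds a current growable and tracks its growth stage.
; SetCurrentGrowable loads the growable from the data table row linked on an input item.
; Events set or increment the stage up to a limit, printing when out of range, while ResetGrowthStage zeroes the limit rather than the stage.
; CompileGrowthStages rebuilds GrowthGraphics from loop indices up to that limit.
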(event Custom|ResetGrowthStage
  (Variables|Default|SetGrowthStageLimit 0))

(event Custom|SetGrowthStage
  (params (New%20Growth%20Stage :type Integer))
  (if (<= New%20Growth%20Stage (Variables|Default|GetGrowthStageLimit))
    (Variables|Default|SetCurrentGrowthStage New%20Growth%20Stage)
    (else
      (Development|PrintString "Given number to set growth stage is larger than limit"))))

(event Custom|IncrementGrowthStage
  (if (< (Variables|Default|GetCurrentGrowthStage) (Variables|Default|GetGrowthStageLimit))
    (bind _result (Math|Integer|IncrementInt (Variables|Default|GetCurrentGrowthStage))
      (:%20%20
        (Variables|Default|SetCurrentGrowthStage _result)))
    (else
      (Development|PrintString "Didin't increment growth stage, is already at limit"))))

(event Custom|CompileGrowthStages
  (Variables|Default|SetGrowthGraphics (Utilities|Array|MakeArray))
  (for _index (range 0 (- (Variables|Default|GetGrowthStageLimit) 0))
    (Utilities|Array|AppendArray (Variables|Default|GetGrowthGraphics) (Utilities|Array|MakeArray 0))))

(event Custom|SetGrowthStageLimit
  (params (New%20Growth%20Stage%20Limit :type Integer))
  (Variables|Default|SetGrowthStageLimit New%20Growth%20Stage%20Limit))

(event Custom|SetCurrentGrowable
  (params (ItemInput :type S%20Item%20Structure))
  (bind _linkedgrowable (Utilities|Struct|BreaksItem ItemInput))
  (bind (_datatable _rowname) (Utilities|Struct|BreakDataTableRowHandle _linkedgrowable))
  (bind _returnvalue (Utilities|GetDataTableRow _datatable _rowname)
    (:then
      (if (!= _rowname "NULL")
        (Variables|Default|SetCurrentGrowable _returnvalue)))))

(fn ConstructionScript
  (Development|PrintString "Hello"))