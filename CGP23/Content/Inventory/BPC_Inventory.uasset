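; Inventory Blueprint component that stores item stacks in an array and takes in new items by merging them into existing stacks.
; TryAddToStack finds the first stack with a matching item name and moves units one at a time until MaxStack or none remain.
; Leftovers go to AddNewStack, a stub that returns false.
; AddItemToInventory calls TryAddToStack but always returns false, and unmatched items never reach AddNewStack.
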(fn AddItemtoInventory
  (params (inItemData :type S%20Item%20Structure))
  (CallFunction|TryAddtoStack inItemData)
  (return false))

(fn TryAddtoStack
  (params (ItemData :type S%20Item%20Structure%20%28by%20ref%29))
  (bind (_itemname _texture _amount) (Utilities|Struct|BreaksItem ItemData))
  (bind _returnvalue (> _amount 0))
  (for (_array_element _array_index) (Variables|Default|GetInventory) ; loop through all stacks
    (if (Utilities|Enum|Equal(Enum) _itemname (.ItemName (Utilities|Struct|BreaksItem _array_element))) ; if one is found which items have the same name as incoming
      (while (and _returnvalue (< (.Amount (Utilities|Struct|BreaksItem _array_element)) (.MaxStack (Utilities|Struct|BreaksItem _array_element)))) ; begin transfer of stack
        (Utilities|Struct|SetmembersinsItem ItemData (- (.Amount (Utilities|Struct|BreaksItem ItemData)) 1))
        (bind _structout (Utilities|Struct|SetmembersinsItem _array_element (+ (.Amount (Utilities|Struct|BreaksItem _array_element)) 1)))
        (Utilities|Array|SetArrayElem (Variables|Default|GetInventory) _array_index _structout))
      (if _returnvalue ; if there is any left
        (bind _success (CallFunction|AddNewStack))
        (return _success)
        (else
          (return true))))))

(fn AddNewStack
  (params (ItemData :type S%20Item%20Structure))
  (return false))