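; BP_FenceSpline is a modular environment actor that builds a fence along an editable spline.
; The construction script derives segment length from the fence mesh's X bounds, then adds enough collision-enabled, X-forward spline mesh components to cover the spline.
; Each segment takes its endpoints and tangents from distances along the spline, with tangent size capped at the segment length.
; The event graph holds no active logic.
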(event EventBeginPlay)

(event Collision|EventActorBeginOverlap
  (params (OtherActor :type Actor%20Object%20Reference)))

(event EventTick
  (params (DeltaSeconds :type Float%20%28single-precision%29)))

(fn ConstructionScript
  (bind _fencemesh (Variables|Components|GetFenceMesh))
  (bind _spline (Variables|Default|GetSpline))
  (bind _returnvalue (StaticMesh|GetBoundingBox _fencemesh))
  (bind _output_get (Variables|Components|SetXLength (.x (+ (Math|Vector|VectorGetAbs (.min _returnvalue)) (Math|Vector|VectorGetAbs (.max _returnvalue))))))
  (for _index (range 0 (Math|Float|Truncate (/ (Spline|GetSplineLength (Variables|Default|GetSpline)) _output_get)))
    (bind _returnvalue_2 (AddComponent|AddSplineMeshComponent false))
    (Collision|SetCollisionEnabled _returnvalue_2 "QueryAndPhysics")
    (SplineMesh|SetForwardAxis _returnvalue_2 "X" true)
    (Components|StaticMesh|SetStaticMesh _returnvalue_2 (Variables|Components|GetFenceMesh))
    (SplineMesh|SetStartandEnd _returnvalue_2 (Spline|GetLocationatDistanceAlongSpline _spline (* _index (Variables|Components|GetXLength)) "Local") (Math|Vector|ClampVectorSize (Spline|GetTangentatDistanceAlongSpline _spline (* _index (Variables|Components|GetXLength)) "Local") 0.0 (Variables|Components|GetXLength)) (Spline|GetLocationatDistanceAlongSpline _spline (* (Variables|Components|GetXLength) (+ _index 1)) "Local") (Math|Vector|ClampVectorSize (Spline|GetTangentatDistanceAlongSpline _spline (* (Variables|Components|GetXLength) (+ _index 1)) "Local") 0.0 (Variables|Components|GetXLength)) true :!class /Script/Engine.SplineMeshComponent)))