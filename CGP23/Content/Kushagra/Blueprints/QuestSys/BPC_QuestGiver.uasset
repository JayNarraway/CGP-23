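; Quest giver component that offers its owner's assigned quest to the player on interaction.
; QuestInteraction asks the player character's quest log component whether the QuestData row is already active, returning the owner's display name either way.
; If inactive, DisplayQuest looks up the data table row and passes it to a new W_QuestGiver widget on the viewport.
; An already active quest only prints a message.
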(event EventBeginPlay)

(event EventTick
  (params (DeltaSeconds :type Float%20%28single-precision%29)))

(fn DisplayQuest
  (bind _questdata (Variables|Default|GetQuestData))
  (bind (_datatable _rowname) (Utilities|Struct|BreakDataTableRowHandle _questdata))
  (bind _returnvalue (Utilities|GetDataTableRow _datatable _rowname)
    (:then
      (bind _returnvalue_2 (UserInterface|CreateWidget "/Game/Kushagra/UI/W_QuestGiver.W_QuestGiver_C" 0 _returnvalue))
      (UserInterface|Viewport|AddtoViewport _returnvalue_2 0)
      (Development|PrintString (Utilities|String|ToString(Text) (.QuestName (Utilities|Struct|BreakS_QuestDetails _returnvalue)))))))

(fn QuestInteraction
  (bind _returnvalue (Components|GetOwner))
  (bind _returnvalue_2 (Utilities|GetDisplayName _returnvalue))
  (if (not (Default|QueryActiveQuest (Variables|/Game/Player/_PLAYER._PLAYER_C|GetBPC_QuestLogComponent (CallFunction|GetPlayerCharacterRef)) (.rowname (Variables|Default|GetQuestData))))
    (CallFunction|DisplayQuest)
    (return _returnvalue_2)
    (else
      (Development|PrintString "Already On Quest!! " true true "(R=1.000000,G=0.026724,B=0.116388,A=1.000000)")
      (return _returnvalue_2))))