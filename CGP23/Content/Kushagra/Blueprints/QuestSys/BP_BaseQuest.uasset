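; BP_BaseQuest is a base quest Blueprint that tracks objective progress for one stage of a data-driven quest.
; GetQuestDetails loads the DT_QuestData row for QuestID, caches the current stage and zeroes a progress map keyed by ObjectiveID.
; On BeginPlay it binds to the player character's objective-ID event; the handler increments matching objectives up to their required quantity.
; Stage advancement and completion are not handled here.
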(event EventBeginPlay
  (EventDispatchers|BindEventtoOnObjectiveIDCalled (CallFunction|GetPlayerCharacterRef) (EventDispatchers|CreateEvent :!event OnObjectiveIDHeard)))

(fn ConstructionScript)

(fn OnObjectiveIDHeard
  (params (ObjectiveID :type String))
  (bind _currentobjectiveprogress (Variables|Default|GetCurrentObjectiveProgress))
  (bind (_value _returnvalue) (Utilities|Map|Find _currentobjectiveprogress ObjectiveID))
  (if _returnvalue
    (if (< _value (.Quantity (Utilities|Struct|BreakS_ObjectiveDetails (CallFunction|GetObjectiveDatabyID ObjectiveID))))
      (Utilities|Map|Add (Variables|Default|GetCurrentObjectiveProgress) ObjectiveID (+ _value 1))
      (return))
    (else
      (return))))

(fn GetQuestDetails
  ;[1 1 1] Basically anytime you want to access the quest data just pull this up
  (bind _returnvalue (Utilities|GetDataTableRow "/Game/Kushagra/Blueprints/QuestSys/DT_QuestData.DT_QuestData" (Variables|Default|GetQuestID))
    (:then
      ;[1 1 1] For referencing elsewhere in the blueprint
      (bind _output_get (Variables|Default|SetQuestDetails _returnvalue))
      (bind _output_get_2 (Variables|Default|SetCurrentStageDetails (Utilities|Array|Get(acopy) (Utilities|Struct|BreakS_QuestDetails _output_get) (Variables|Default|GetCurrentStage))))
      (Utilities|Map|Clear (Variables|Default|GetCurrentObjectiveProgress))
      (for _array_element (Utilities|Struct|BreakS_StageDetails _output_get_2)
        (Utilities|Map|Add (Variables|Default|GetCurrentObjectiveProgress) (Utilities|Struct|BreakS_ObjectiveDetails _array_element) 0)))))

(fn GetObjectiveDatabyID
  (params (ObjectiveID :type String))
  (for _array_element (.Objectives (Utilities|Struct|BreakS_StageDetails (Variables|Default|GetCurrentStageDetails)))
    (if (Utilities|Enum|Equal(Enum) (.ObjectiveID (Utilities|Struct|BreakS_ObjectiveDetails _array_element)) ObjectiveID)
      (return _array_element))))