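; Build-mode component for BP_TopDownCharacter that previews and spawns buildables loaded from DT_Buildables at BeginPlay.
; While build mode is on, BuildCycle and a short BuildDelay loop as a custom tick, tracing from the mouse cursor toward a grid-snapped end point.
; The trace moves a collisionless ghost mesh, tinted green on a hit and red on a miss.
; SpawnBuild spawns the selected actor at that transform without checking CanBuild.
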(event Custom|BuildDelay
  (bind _buildghost (Variables|Default|GetBuildGhost))
  (if (Variables|Default|GetIsBuildModeOn?)
    ;[1 1 1] This is basically a self made event tick and that Delay Value Duration decides how many times do we wanna run it
    (Utilities|FlowControl|Delay 0.01)
    (CallFunction|BuildCycle)
    (else
      (Variables|Default|SetIsBuildModeOn? false)
      (Variables|Default|SetCanBuild? false)
      (Utilities|IsValid _buildghost
        (:Is%20Valid
          (Default|DestroyComponent (Variables|Default|GetTopDownCharacterRef) _buildghost))))))

(event Custom|StopBuildMode
  (bind _buildghost (Variables|Default|GetBuildGhost))
  (Variables|Default|SetIsBuildModeOn? false)
  (Variables|Default|SetCanBuild? false)
  (Utilities|IsValid _buildghost
    (:Is%20Valid
      (Default|DestroyComponent (Variables|Default|GetTopDownCharacterRef) _buildghost))))

(event Custom|LaunchBuildMode
  (if (Variables|Default|GetIsBuildModeOn?)
    (CallFunction|StopBuildMode)
    (else
      (Variables|Default|SetIsBuildModeOn? true)
      (CallFunction|BuildCycle))))

(event EventBeginPlay
  ;[1 1 1] Make sure correct refs and not dupicating casue IT WILL CRASH
  (bind _asbp_top_down_character (Utilities|Casting|CastToBP_TopDownCharacter (Components|GetOwner)))
  (Variables|Default|SetTopDownCharacterRef _asbp_top_down_character)
  (bind _outrownames (DataTable|GetDataTableRowNames "/Game/Kushagra/Blueprints/DT_Buildables.DT_Buildables"))
  (for _array_element _outrownames
    (bind _returnvalue (Utilities|GetDataTableRow "/Game/Kushagra/Blueprints/DT_Buildables.DT_Buildables" _array_element)
      (:then
        (Utilities|Array|Add (Variables|Default|GetStructBuildables) _returnvalue)))))

(fn SpawnBuildGhost
  (bind _returnvalue (Game|AddComponentbyClass (Variables|Default|GetTopDownCharacterRef) "/Script/Engine.StaticMeshComponent" false (Variables|Default|GetBuildTransform)))
  (bind _output_get (Variables|Default|SetBuildGhost _returnvalue))
  (Components|StaticMesh|SetStaticMesh _output_get (.Mesh (Utilities|Struct|BreakS_Buildables (Utilities|Array|Get(acopy) (Variables|Default|GetStructBuildables) (Variables|Default|GetBuildID)))))
  ;[1 1 1] So that you do not collide with the build ghost
  (Collision|SetCollisionEnabled (Variables|Default|GetBuildGhost) "NoCollision"))

(fn GiveBuildColor
  (params (IsGreen? :type Boolean))
  (bind _buildghost (Variables|Default|GetBuildGhost))
  ;[0.01938 0.01938 0.01938] Can Build is not used for the branch
  (Variables|Default|SetCanBuild? IsGreen?)
  (if IsGreen?
    (Rendering|Material|SetMaterial _buildghost 0 "/Game/Kushagra/Assets/Materials/MI_TransGreen.MI_TransGreen")
    (else
      (Rendering|Material|SetMaterial _buildghost 0 "/Game/Kushagra/Assets/Materials/MI_TransRed.MI_TransRed")))
  (Transformation|SetWorldTransform (Variables|Default|GetBuildGhost) (Variables|Default|GetBuildTransform) false false))

(fn BuildCycle
  (bind _returnvalue (Game|GetPlayerController 0))
  (bind _buildghost (Variables|Default|GetBuildGhost))
  (bind (_worldlocation _worlddirection) (Game|Player|ConvertMouseLocationToWorldSpace _returnvalue))
  ;[1 1 1] This is for camera based line-trace but the game is top-down isometric so pls change to cursor
  (bind (_outhit _returnvalue_2) (Collision|LineTraceByChannel _worldlocation (Class|KismetMathLibrary|VectorSnappedtoGrid (+ _worldlocation (* _worlddirection 2500)) 2.5e+02) (.tracechannel (Utilities|Array|Get(acopy) (Variables|Default|GetStructBuildables) (Variables|Default|GetBuildID))) false 0 "ForDuration" true "(R=1.000000,G=0.000000,B=0.000000,A=1.000000)" "(R=0.000000,G=1.000000,B=0.000000,A=1.000000)" 2.0))
  (if _returnvalue_2
    (Variables|Default|SetBuildTransform (Math|Transform|MakeTransform (.ImpactPoint (Collision|BreakHitResult _outhit)) (.rotation (Variables|Default|GetBuildTransform)) (.scale (Variables|Default|GetBuildTransform))))
    (Utilities|IsValid _buildghost
      (:Is%20Valid
        (CallFunction|GiveBuildColor true))
      (:Is%20Not%20Valid
        (CallFunction|SpawnBuildGhost :!label _label)))
    (else
      (Variables|Default|SetBuildTransform (Math|Transform|MakeTransform (.TraceEnd (Collision|BreakHitResult _outhit)) (.rotation (Variables|Default|GetBuildTransform)) (.scale (Variables|Default|GetBuildTransform))))
      (Utilities|IsValid _buildghost
        (:Is%20Valid
          (CallFunction|GiveBuildColor false))
        (:Is%20Not%20Valid
          (goto _label)))))
  (CallFunction|BuildDelay))

(fn ChangeMesh
  (Components|StaticMesh|SetStaticMesh (Variables|Default|GetBuildGhost) (.mesh (Utilities|Array|Get(acopy) (Variables|Default|GetStructBuildables) (Variables|Default|GetBuildID)))))

(fn SpawnBuild
  (Game|SpawnActorfromClass (.actor (Utilities|Array|Get(acopy) (Variables|Default|GetStructBuildables) (Variables|Default|GetBuildID))) (Variables|Default|GetBuildTransform) "Undefined" "MultiplyWithRoot" 0 0))