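; Component that runs a cooking stir quick-time event, where the player holds left or right to match a randomly timed, flipping direction.
; StartCooking consumes the item, swaps input to IMC_QTE and shows WB_CycleQTE.
; Tick drives StirringLoop: holding correctly allows flips toward success, while releasing builds BoilTimer toward failure.
; Either ending restores perspective and adds the pot-data output item, as SpawnItem's burned-food selection is unconnected.
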(event Custom|StartCooking
  (params (TotalFlips :type Byte) (OverCookedTime :type Float%20%28double-precision%29) (FlipTimeMax :type Float%20%28double-precision%29) (FlipTimeMin :type Float%20%28double-precision%29) (InteractedItem :type S%20Item%20Structure))
  (bind _returnvalue (Game|GetPlayerController 0))
  (bind _widget (Variables|Default|Getwidget))
  (bind _returnvalue_2 (PlayerController|LocalPlayerSubsystems|GetEnhancedInputLocalPlayerSubsystem _returnvalue))
  (bind _success (CallFunction|HandleItemin InteractedItem))
  ;[1 0.5473 0.01173] Start
  (if _success
    (Variables|Default|SetRunning true)
    (Variables|Default|SetFlipTotal TotalFlips)
    (Variables|Default|SetFailTime OverCookedTime)
    (Variables|Default|SetSwitchTimerMax FlipTimeMax)
    (Variables|Default|SetSwitchTimerMin FlipTimeMin)
    (Input|RemoveMappingContext _returnvalue_2 "/Game/Tech/Core/Input/IMC_2D.IMC_2D" "(bIgnoreAllPressedKeysUntilRelease=True,bForceImmediately=False)")
    (Input|RemoveMappingContext _returnvalue_2 "/Game/Tech/Core/Input/IMC_ISO.IMC_ISO" "(bIgnoreAllPressedKeysUntilRelease=True,bForceImmediately=False)")
    (Input|AddMappingContext _returnvalue_2 "/Game/Tech/Core/Input/IMC_QTE.IMC_QTE" 0 "(bIgnoreAllPressedKeysUntilRelease=True,bForceImmediately=False)")
    (Variables|Default|SetClockwise (Math|Random|RandomBool))
    (Variables|Default|SetFlipAt (Math|Random|RandomFloatinRange (Variables|Default|GetSwitchTimerMin) (Variables|Default|GetSwitchTimerMax)))
    (Components|Tick|SetComponentTickEnabled true)
    (Default|FlipImage _widget (not (Variables|Default|GetClockwise)))
    (UserInterface|Viewport|AddtoViewport _widget 0)))

(event Custom|End
  ;[1 0 0.01829] End
  (Default|ReturnPerspective (Variables|Default|GetAs%20CONTROLLER) true)
  (Components|Tick|SetComponentTickEnabled false)
  (Variables|Default|SetTimer 0.0)
  (Variables|Default|SetFlipAt 0.0)
  (Variables|Default|SetFlipCount 0)
  (Variables|Default|SetBoilTimer 0.0)
  (Widget|RemovefromParent (Variables|Default|Getwidget))
  (Variables|Default|SetRunning false))

(event Custom|Flip
  ;[1 0 0.8683] Flip
  (bind _output_get (Variables|Default|SetFlipCount (+ (Variables|Default|GetFlipCount) 1)))
  (if (>= _output_get (Variables|Default|GetFlipTotal))
    (Development|PrintString "success")
    (CallFunction|SpawnItem true)
    (CallFunction|End)
    (else
      (bind _output_get_2 (Variables|Default|SetClockwise (not (Variables|Default|GetClockwise))))
      (Default|FlipImage (Variables|Default|Getwidget) (not _output_get_2))
      (Variables|Default|SetTimer 0.0)
      (Variables|Default|SetFlipAt (Math|Random|RandomFloatinRange (Variables|Default|GetSwitchTimerMin) (Variables|Default|GetSwitchTimerMax))))))

(event Input|EnhancedActionEvents|EnhancedInputActionIA_Left
  (params (ActionValue :type Boolean) (ElapsedSeconds :type Float%20%28double-precision%29) (TriggeredSeconds :type Float%20%28double-precision%29) (InputAction :type Input%20Action%20Object%20Reference :default "/Game/Tech/Core/Input/Actions/QTEActions/IA_Left.IA_Left"))
  (bind _widget (Variables|Default|Getwidget))
  (bind _running (Variables|Default|GetRunning))
  ;[0 0.9624 1] Input
  (:Triggered
    (if _running :!label _label
      (Variables|Default|SetLeftHeld ActionValue)
      (Default|MoveThrobber _widget _running true)))
  (:Completed
    (Default|MoveThrobber _widget false true)
    (goto _label)))

(event Input|EnhancedActionEvents|EnhancedInputActionIA_Right
  (params (ActionValue :type Boolean) (ElapsedSeconds :type Float%20%28double-precision%29) (TriggeredSeconds :type Float%20%28double-precision%29) (InputAction :type Input%20Action%20Object%20Reference :default "/Game/Tech/Core/Input/Actions/QTEActions/IA_Right.IA_Right"))
  (bind _widget (Variables|Default|Getwidget))
  (bind _running (Variables|Default|GetRunning))
  ;[0 0.9624 1] Input
  (:Triggered
    (if _running :!label _label
      (Variables|Default|SetRightHeld ActionValue)
      (Default|MoveThrobber _widget _running false)))
  (:Completed
    (Default|MoveThrobber _widget false false)
    (goto _label)))

(event EventBeginPlay
  ;[0.1444 1 0] Begin Play
  (bind _returnvalue (UserInterface|CreateWidget "/Game/Tech/QTE/WB_CycleQTE.WB_CycleQTE_C" (Game|GetPlayerController 0)))
  (Variables|Default|Setwidget _returnvalue)
  (bind _as_controller (Utilities|Casting|CastTo_CONTROLLER (Game|GetPlayerController 0)))
  (Variables|Default|SetAs%20CONTROLLER _as_controller))

(event EventTick
  (params (DeltaSeconds :type Float%20%28single-precision%29))
  ;[0 0.884 1] Update
  (Variables|Default|SetTimer (+ DeltaSeconds (Variables|Default|GetTimer)))
  (if (Variables|Default|GetClockwise)
    (CallFunction|StirringLoop (Variables|Default|GetRightHeld))
    (Development|PrintString "right" true false "(R=0.000000,G=0.045587,B=1.000000,A=1.000000)" 2.0 "QTE_Right")
    (else
      (CallFunction|StirringLoop (Variables|Default|GetLeftHeld))
      (Development|PrintString "Left" true false "(R=0.330907,G=0.000000,B=1.000000,A=1.000000)" 2.0 "QTE_Left"))))

(fn StirringLoop
  (params (Held :type Boolean))
  (if Held
    ;[0 1 0.9709] Check for flip
    (if (<= (Variables|Default|GetBoilTimer) 0.0)
      (Variables|Default|SetBoilTimer 0.0)
      (else
        (Variables|Default|SetBoilTimer (- (Utilities|Time|GetWorldDeltaSeconds) (Variables|Default|GetBoilTimer)))))
    (if (>= (Variables|Default|GetTimer) (Variables|Default|GetFlipAt))
      (CallFunction|Flip))
    (else
      ;[1 0.02435 0] Check if fail
      (Variables|Default|SetBoilTimer (+ (Variables|Default|GetBoilTimer) (Utilities|Time|GetWorldDeltaSeconds)))
      (if (>= (Variables|Default|GetBoilTimer) (Variables|Default|GetFailTime))
        (Development|PrintString "Fail")
        (CallFunction|SpawnItem false)
        (CallFunction|End)))))

(fn SpawnItem
  (params (isSuccess :type Boolean))
  (bind _in_item (Variables|Default|GetIn%20Item))
  (bind (_itemname _texture _amount_shouldbe1 _isstackable _maxstack _mesh _linkedgrowdata _linkedovendata _linkedpotdata _linkedchopdata _itemquality_ignore _owninginventory_ignore) (Utilities|Struct|BreaksItem _in_item))
  (bind (_datatable _rowname) (Utilities|Struct|BreakDataTableRowHandle _linkedpotdata))
  (bind _returnvalue (Utilities|GetDataTableRow _datatable _rowname)
    (:then
      (bind _returnvalue_2 (Utilities|GetDataTableRow (.DataTable (Utilities|Struct|BreakDataTableRowHandle (.OutputItem (Utilities|Struct|BreaksFood _returnvalue)))) (.RowName (Utilities|Struct|BreakDataTableRowHandle (.OutputItem (Utilities|Struct|BreaksFood _returnvalue)))))
        (:then
          (Default|AddItemtoInventory _owninginventory_ignore _returnvalue_2))))))

(fn HandleItemin
  (params (InItem :type S%20Item%20Structure))
  (bind (_itemname _texture _amount_shouldbe1 _isstackable _maxstack _mesh _linkedgrowdata _linkedovendata _linkedpotdata) (Utilities|Struct|BreaksItem InItem))
  (if (Utilities|Enum|Equal(Enum) _itemname (Utilities|Text|MakeLiteralText "AIR"))
    _
    (elif (not (== (.RowName (Utilities|Struct|BreakDataTableRowHandle _linkedpotdata)) "EMPTY"))
      (bind _output_get (Variables|Default|SetIn%20Item InItem))
      (bind _itemremoved (Default|RemoveItem (.OwningInventory-IGNORE (Utilities|Struct|BreaksItem _output_get)) _output_get))
      (if _itemremoved
        (return true)
        (else
          (return false)))
      (else
        _)))
  (return false))