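; BP_CameraZone is a trigger volume that switches the player's camera when the player enters it.
; On box overlap, it calls ChangeCamera on the _PLAYER, passing its isometric flag, the TPLocator world position and a reference to itself.
; A separate ToggleVis event, not called within this Blueprint, flips visibility and updates collision on a list of assigned actors.
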(event OnComponentBeginOverlap(Box)
  (params (OverlappedComponent :type Primitive%20Component%20Object%20Reference) (OtherActor :type Actor%20Object%20Reference) (OtherComp :type Primitive%20Component%20Object%20Reference) (OtherBodyIndex :type Integer) (bFromSweep :type Boolean) (SweepResult :type Hit%20Result%20Structure%20%28by%20ref%29))
  (bind _as_player (Utilities|Casting|CastTo_PLAYER OtherActor))
  (Default|ChangeCamera _as_player (Variables|Default|GetisIso) (Transformation|GetWorldLocation (Variables|Default|GetTPLocator)) self false))

(event Custom|ToggleVis
  (for _array_element (Variables|Default|GetAssetsToToggleVisibility)
    (Utilities|IsValid _array_element
      (:Is%20Valid
        (Rendering|SetActorHiddenInGame _array_element (not (Variables|/Script/Engine.Actor|GetbHidden _array_element)))
        (Collision|SetActorEnableCollision _array_element (not (Variables|/Script/Engine.Actor|GetbHidden _array_element)))))))

(fn ConstructionScript)