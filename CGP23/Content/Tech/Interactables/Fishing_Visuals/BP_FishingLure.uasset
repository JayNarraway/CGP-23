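; Fishing lure actor that launches itself forward from the player on spawn and signals fish state through its colour.
; On BeginPlay it applies a velocity-change impulse to its Sphere along the player capsule's forward vector.
; A dynamic material created in the construction script starts bright red, turns bright green on FishReady and resets to MakeColor's default on FishGone, rather than back to red.
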(event EventBeginPlay
  (bind _sphere (Variables|Default|GetSphere))
  (bind _returnvalue (Actor|GetActorOfClass "/Game/Tech/Core/Player(Proto)/_PLAYER._PLAYER_C"))
  (bind _as_player (Utilities|Casting|CastTo_PLAYER _returnvalue))
  (Class|PrimitiveComponent|AddVelocityChangeImpulseatLocation _sphere (* (Math|Vector|GetForwardVector (Variables|/Script/Engine.Character|GetCapsuleComponent _as_player)) "200.000000,200.000000,200.000000") (Variables|/Script/Engine.SceneComponent|GetRelativeLocation _sphere) "None"))

(event EventFishReady
  (Rendering|Material|SetVectorParameterValue (Variables|Default|GetMaterialColour) "Colour" (Math|Color|MakeColor 0.0 1e+04 0.0) :!class /Script/Engine.MaterialInstanceDynamic))

(event EventFishGone
  (Rendering|Material|SetVectorParameterValue (Variables|Default|GetMaterialColour) "Colour" (Math|Color|MakeColor 0.0 0.0 0.0) :!class /Script/Engine.MaterialInstanceDynamic))

(fn ConstructionScript
  (bind _returnvalue (Rendering|Material|CreateDynamicMaterialInstance (Variables|Default|GetSphere) 0 0 "None" :!class /Script/Engine.PrimitiveComponent))
  (bind _output_get (Variables|Default|SetMaterialColour _returnvalue))
  (Rendering|Material|SetVectorParameterValue _output_get "Colour" (Math|Color|MakeColor 1e+04 0.0 0.0) :!class /Script/Engine.MaterialInstanceDynamic))