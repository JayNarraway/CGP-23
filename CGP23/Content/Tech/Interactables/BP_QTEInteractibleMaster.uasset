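; Master Blueprint for interactables that use quick time events (QTE), serving as a base with placeholder success and fail responses.
; On BeginPlay it binds delegates to the success and fail events of its BPCQTELogic component.
; Its QTESuccess and QTEFail events only print debug messages, and its construction script just calls the parent.
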(event Custom|QTESuccess
  (Development|PrintString "QTE Success!"))

(event Custom|QTEFail
  (Development|PrintString "QTE Fail!"))

(event EventBeginPlay
  (bind _bpc_qtelogic (Variables|Default|GetBPC_QTELogic))
  (EventDispatchers|BindEventtoQTESuccess _bpc_qtelogic (EventDispatchers|CreateEvent :!event Custom|QTESuccess))
  (EventDispatchers|BindEventtoQTEFail _bpc_qtelogic (EventDispatchers|CreateEvent :!event Custom|QTEFail)))

(fn ConstructionScript
  (|CallParentFunction))