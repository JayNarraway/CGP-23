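; BP_CropPlot is an interactable plot that grows a plant from a held item and yields an item when harvested.
; Each interaction first tries a harvest, then looks up the held item's grow data row, plants it and removes the item from its inventory.
; A one-shot timer ends growth while a looping timer scales the mesh by elapsed time.
; Harvesting a grown plant spawns a BP_BaseItem and resets the plot.
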(event Custom|BeginGrowth
  (Transformation|SetRelativeScale3D (Variables|Default|GetPlant) "0, 0, 0")
  (Variables|Default|SetisGrowing true)
  (bind _returnvalue (Utilities|Time|SetTimerbyEvent (delegate Custom|FinishedGrowth) (.GrowTime (Utilities|Struct|BreaksGrowable (Variables|Default|GetCurrentGrowingItem)))))
  (bind _returnvalue_2 (Utilities|Time|SetTimerbyEvent (delegate Custom|HandleScale) (Variables|Default|GetTickRate) true)))

(event Custom|HandleScale
  (bind _output_get (Variables|Default|SetGrowthPercentage (/ (Class|KismetSystemLibrary|GetTimerElapsedTimeHandle (stale Custom|BeginGrowth _returnvalue)) (.GrowTime (Utilities|Struct|BreaksGrowable (Variables|Default|GetCurrentGrowingItem))))))
  (Transformation|SetRelativeScale3D (Variables|Default|GetPlant) (Math|Vector|Lerp(Vector) "0, 0, 0" "1.000000,1.000000,1.000000" _output_get)))

(event Custom|FinishedGrowth
  (Utilities|Time|ClearandInvalidateTimerbyHandle (stale Custom|BeginGrowth _returnvalue_2))
  (Variables|Default|SetisGrowing false))

(fn ConstructionScript
  (|CallParentFunction))

(fn AttemptHarvest
  (if (and (>= (Variables|Default|GetGrowthPercentage) 0.98) (not (Variables|Default|GetisGrowing)))
    (CallFunction|SpawnItem (.GrownItem (Utilities|Struct|BreaksGrowable (Variables|Default|GetCurrentGrowingItem))))
    (Transformation|SetRelativeScale3D (Variables|Default|GetPlant) "0, 0, 0")
    (Variables|Default|SetCurrentGrowingItem "")
    (Variables|Default|SetGrowthPercentage 0.0)
    (else
      (Development|PrintString "Not Ready For Harvest"))))

(fn AttemptPlant
  (params (inGrowable :type S%20Growable%20Structure))
  (bind (_plantname _mesh) (Utilities|Struct|BreaksGrowable inGrowable))
  (if (Variables|Default|GetisGrowing)
    (Development|PrintString "Something is Growing!" true true "(R=1.000000,G=0.000000,B=0.000000,A=1.000000)")
    (return false)
    (else
      (Components|StaticMesh|SetStaticMesh (Variables|Default|GetPlant) _mesh)
      (Variables|Default|SetCurrentGrowingItem inGrowable)
      (CallFunction|BeginGrowth)
      (Development|PrintString (Utilities|String|Append "Planted: " (Utilities|String|ToString(Text) _plantname)) true true "(R=0.000000,G=1.000000,B=0.093997,A=1.000000)")
      (return true))))

(fn SpawnItem
  (params (inItem :type Data%20Table%20Row%20Handle%20Structure))
  (Game|SpawnActorfromClass "/Game/Tech/Inventory/BP_BaseItem.BP_BaseItem_C" (Math|Transform|MakeTransform (Transformation|GetWorldLocation (Variables|Default|GetItemSpawnPoint)) "0, 0, 0" "1.000000,1.000000,1.000000") "Undefined" "MultiplyWithRoot" 0 inItem 0))

(fn InteractionwithHeldItem
  (params (ItemInHand :type S%20Item%20Structure))
  (bind (_itemname _texture _amount_shouldbe1 _isstackable _maxstack _mesh _linkedgrowdata) (Utilities|Struct|BreaksItem ItemInHand))
  (bind (_datatable _rowname) (Utilities|Struct|BreakDataTableRowHandle _linkedgrowdata))
  (CallFunction|AttemptHarvest)
  (if (Utilities|Enum|Equal(Enum) _itemname (Utilities|Text|MakeLiteralText "AIR"))
    (Development|PrintString "Empty Hand")
    (elif (== _rowname "EMPTY")
      (Development|PrintString "NO PLANT ASSOCIATED")
      (else
        (bind _returnvalue (Utilities|GetDataTableRow _datatable _rowname)
          (:then
            (Development|PrintString (Utilities|String|Append "Attempting to Grow: " (Utilities|String|ToString(Name) _rowname)))
            (bind _isplanted (CallFunction|AttemptPlant _returnvalue))
            (if _isplanted
              (Default|RemoveItem (.OwningInventory-IGNORE (Utilities|Struct|BreaksItem ItemInHand)) ItemInHand))))))))