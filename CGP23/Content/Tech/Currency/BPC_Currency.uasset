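; Blueprint component that stores a currency balance in Drachmas for the game.
; ChangeCurrency adds an amount to the balance and clamps the result to a fixed range from zero to a cap.
; SetCurrency overwrites the balance directly without clamping, and GetCurrency returns the current value.
; It has no active event logic, so the balance changes only when these functions are called.
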(event EventBeginPlay)

(event EventTick
  (params (DeltaSeconds :type Float%20%28single-precision%29)))

(fn ChangeCurrency
  (params (Amount :type Integer))
  (bind _output_get (Variables|Default|SetDrachmas (Math|Integer|Clamp(Integer) (+ Amount (Variables|Default|GetDrachmas)) 0 10000)))
  (return _output_get))

(fn GetCurrency
  (return (Variables|Default|GetDrachmas)))

(fn SetCurrency
  (params (New%20Currency :type Integer))
  (bind _output_get (Variables|Default|SetDrachmas New%20Currency))
  (return _output_get))