(event Custom|BuildDelay
  (bind _buildghost (Variables|Default|GetBuildGhost))
  (if (Variables|Default|GetIsBuildModeOn?)
    ;[1 1 1] This is basically a self made event tick and that Delay Value Duration decides how many times do we wanna run it
    (Utilities|FlowControl|Delay 0.01)
    (CallFunction|BuildCycle)
    (else
      (Variables|Default|SetIsBuildModeOn? false)
      (Variables|Default|SetCanBuild? false)
      (Utilities|IsValid _buildghost
        (:Is%20Valid
          (Default|DestroyComponent (Variables|Default|GetPLAYER_REF) _buildghost))))))

(event Custom|StopBuildMode
  (bind _buildghost (Variables|Default|GetBuildGhost))
  (Variables|Default|SetIsBuildModeOn? false)
  (Variables|Default|SetCanBuild? false)
  (Utilities|IsValid _buildghost
    (:Is%20Valid
      (Default|DestroyComponent (Variables|Default|GetPLAYER_REF) _buildghost))))

(event Custom|LaunchBuildMode
  (bind _returnvalue (Game|GetPlayerController 0))
  (if (Variables|Default|GetIsBuildModeOn?)
    (CallFunction|StopBuildMode)
    (Variables|/Script/Engine.PlayerController|SetbShowMouseCursor _returnvalue false)
    (Input|SetInputModeGameOnly _returnvalue false)
    (else
      (Variables|Default|SetIsBuildModeOn? true)
      (CallFunction|BuildCycle)
      (Variables|/Script/Engine.PlayerController|SetbShowMouseCursor _returnvalue true)
      (Input|SetInputModeGameandUI _returnvalue 0 "DoNotLock" false false))))

(event EventBeginPlay
  ;[1 1 1] Make sure correct refs and not dupicating casue IT WILL CRASH
  (bind _as_player (Utilities|Casting|CastTo_PLAYER (Components|GetOwner)))
  (Variables|Default|SetPLAYER_REF _as_player)
  (bind _outrownames (DataTable|GetDataTableRowNames "/Game/Tech/BuildSystem/Blueprints/DT_Buildables.DT_Buildables"))
  (for _array_element _outrownames
    (bind _returnvalue (Utilities|GetDataTableRow "/Game/Tech/BuildSystem/Blueprints/DT_Buildables.DT_Buildables" _array_element)
      (:then
        (Utilities|Array|Add (Variables|Default|GetStructBuildables) _returnvalue)))))

(fn SpawnBuildGhost
  (bind _returnvalue (Game|AddComponentbyClass (Variables|Default|GetPLAYER_REF) "/Script/Engine.StaticMeshComponent" false (Variables|Default|GetBuildTransform)))
  (bind _output_get (Variables|Default|SetBuildGhost _returnvalue))
  (Components|StaticMesh|SetStaticMesh _output_get (.Mesh (Utilities|Struct|BreakS_Buildables (Utilities|Array|Get(acopy) (Variables|Default|GetStructBuildables) (Variables|Default|GetBuildID)))))
  ;[1 1 1] So that you do not collide with the build ghost
  (Collision|SetCollisionEnabled (Variables|Default|GetBuildGhost) "NoCollision"))

(fn GiveBuildColor
  (params (IsGreen? :type Boolean))
  (bind _buildghost (Variables|Default|GetBuildGhost))
  ;[0.01938 0.01938 0.01938] Can Build is not used for the branch
  (Variables|Default|SetCanBuild? IsGreen?)
  (if IsGreen?
    (Rendering|Material|SetMaterial _buildghost 0 "/Game/Tech/BuildSystem/Assets/Materials/MI_TransGreen.MI_TransGreen")
    (else
      (Rendering|Material|SetMaterial _buildghost 0 "/Game/Tech/BuildSystem/Assets/Materials/MI_TransRed.MI_TransRed")))
  (Transformation|SetWorldTransform (Variables|Default|GetBuildGhost) (Variables|Default|GetBuildTransform) false false))

(fn BuildCycle
  (bind _player_ref (Variables|Default|GetPLAYER_REF))
  (bind _buildghost (Variables|Default|GetBuildGhost))
  (bind _camera (Variables|/Game/Tech/Core/Player(Proto)/_PLAYER._PLAYER_C|GetCamera _player_ref))
  (bind _returnvalue (Transformation|GetWorldLocation _camera))
  (bind (_outhit _returnvalue_2) (Collision|LineTraceByChannel _returnvalue (+ _returnvalue (* (Math|Vector|GetUnitDirection(Vector) _returnvalue (.Location (Collision|BreakHitResult (.HitResult (Game|Player|GetHitResultUnderCursorbyChannel (Game|GetPlayerController 0) "TraceTypeQuery1" true))))) 1e+04)) "TraceTypeQuery1" true 0 "ForOneFrame" true "(R=1.000000,G=0.000000,B=0.000000,A=1.000000)" "(R=0.000000,G=1.000000,B=0.000000,A=1.000000)" 1.0))
  (if _returnvalue_2
    (Variables|Default|SetBuildTransform (Math|Transform|MakeTransform (Class|KismetMathLibrary|VectorSnappedtoGrid (.ImpactPoint (Collision|BreakHitResult _outhit)) 2.5e+02) (.rotation (Variables|Default|GetBuildTransform)) (.scale (Variables|Default|GetBuildTransform))))
    (Variables|BuildCycle|SetHitActor (.HitActor (Collision|BreakHitResult _outhit)))
    (Variables|BuildCycle|SetHit%20Component (.HitComponent (Collision|BreakHitResult _outhit)))
    (Utilities|IsValid _buildghost
      (:Is%20Valid
        (bind (_found _foundtransform) (CallFunction|DetectSnapBoxes))
        (if _found
          (Variables|Default|SetBuildTransform _foundtransform)
          (bind _hit_ (CallFunction|CheckforOverlap))
          (if _hit_
            (CallFunction|GiveBuildColor true :!label _label)
            (else
              (CallFunction|GiveBuildColor false)))
          (else
            (goto _label)))
        (CallFunction|BuildDelay))
      (:Is%20Not%20Valid
        (CallFunction|SpawnBuildGhost :!label _label_2)
        (CallFunction|BuildDelay :!label _label_3)))
    (else
      (Variables|Default|SetBuildTransform (Math|Transform|MakeTransform (Class|KismetMathLibrary|VectorSnappedtoGrid (.TraceEnd (Collision|BreakHitResult _outhit)) 2.5e+02) (.rotation (Variables|Default|GetBuildTransform)) (.scale (Variables|Default|GetBuildTransform))))
      (Utilities|IsValid _buildghost
        (:Is%20Valid
          (CallFunction|GiveBuildColor false)
          (goto _label_3))
        (:Is%20Not%20Valid
          (goto _label_2))))))

(fn ChangeMesh
  (bind _buildghost (Variables|Default|GetBuildGhost))
  (Utilities|IsValid _buildghost
    (:Is%20Valid
      (Components|StaticMesh|SetStaticMesh _buildghost (.mesh (Utilities|Array|Get(acopy) (Variables|Default|GetStructBuildables) (Variables|Default|GetBuildID)))))))

(fn SpawnBuild
  (Game|SpawnActorfromClass (.actor (Utilities|Array|Get(acopy) (Variables|Default|GetStructBuildables) (Variables|Default|GetBuildID))) (Variables|Default|GetBuildTransform) "Undefined" "MultiplyWithRoot" 0 0))

(fn DetectSnapBoxes
  (bind _snapboxesref (Class|BIBuildInterface|ReturnBoxes(Message) (Variables|BuildCycle|GetHitActor)))
  ;[1 1 1] If u find one breka
  (bind _array_element (Utilities|Array|ForEachLoopwithBreak _snapboxesref :!label _label)
    (:LoopBody
      (if (== _array_element (Variables|BuildCycle|GetHit%20Component))
        (LocalVariables|SetLocalFound true)
        (goto _label Break)))
    (:Completed
      (return (LocalVariables|GetLocalFound) (Transformation|GetWorldTransform (Variables|BuildCycle|GetHit%20Component))))))

(fn CheckforOverlap
  (bind _buildghost (Variables|Default|GetBuildGhost))
  (bind (_origin _boxextent) (Collision|GetComponentBounds _buildghost))
  (bind (_outhit _returnvalue) (Collision|BoxTraceByChannel _origin _origin (/ _boxextent 1.02) "0, 0, 0" "TraceTypeQuery1" false 0 "ForOneFrame" true "(R=1.000000,G=0.000000,B=0.000000,A=1.000000)" "(R=0.000000,G=1.000000,B=0.000000,A=1.000000)" 2.0))
  (return _returnvalue))