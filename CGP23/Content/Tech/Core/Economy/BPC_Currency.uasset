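; Currency component that holds a Drachma balance for the game's economy, reset to zero by its Initialise event.
; Set, Get and Change functions manage the balance, with Change clamping to a minimum of zero and no effective upper limit.
; CheckCurrency also spends: it deducts an affordable cost and returns the remainder with CanPurchase, which re-evaluates against the already reduced balance.
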(event Custom|Initialise
  (CallFunction|SetCurrency))

(fn SetCurrency
  (params (New%20Drachma :type Integer))
  (bind _output_get (Variables|Default|SetDrachma New%20Drachma))
  (return _output_get))

(fn CheckCurrency
  (params (Needed%20Drachma :type Integer))
  (if (>= (- (Variables|Default|GetDrachma) Needed%20Drachma) 0)
    (bind _output_get (Variables|Default|SetDrachma (- (Variables|Default|GetDrachma) Needed%20Drachma)))
    (return _output_get (>= (- (Variables|Default|GetDrachma) Needed%20Drachma) 0))
    (else
      (return (Variables|Default|GetDrachma) (>= (- (Variables|Default|GetDrachma) Needed%20Drachma) 0)))))

(fn GetCurrency
  (return (Variables|Default|GetDrachma)))

(fn ChangeCurrency
  (params (Currency%20Change :type Integer))
  (bind _output_get (Variables|Default|SetDrachma (Math|Integer|Clamp(Integer) (+ Currency%20Change (Variables|Default|GetDrachma)) 0 (+ Currency%20Change (Variables|Default|GetDrachma)))))
  (return _output_get))