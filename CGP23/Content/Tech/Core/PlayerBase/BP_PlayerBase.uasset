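; Base player character that handles input for movement, pausing, building, inventory slot selection and interaction.
; Init creates the HUD and caches the player controller, then calls InitCam, which is empty here.
; 2D and 3D moves follow the ForwardVec component, rotate the mesh toward velocity and trigger rubble VFX, marked broken.
; Building delegates to BPCBuildComponent, while interaction box-overlaps interactables and passes them the selected BPCInventory item.
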(event Custom|Init
  ;[1 1 1] Init
  (CallFunction|CreateHUD)
  (Variables|Default|GetPC
    (:then)
    (:else
      (bind _aspc_base (Utilities|Casting|CastToPC_Base (Game|GetPlayerController 0)))
      (Variables|Default|SetPC _aspc_base)
      (CallFunction|InitCam))))

(event Custom|Create%20HUD
  (bind _self self)
  ;[1 1 1] Init
  (bind _returnvalue (UserInterface|CreateWidget "/Game/Design/UI/UI_HUD.UI_HUD_C" 0 _self))
  (Default|Init _returnvalue _self)
  (UserInterface|Viewport|AddtoViewport _returnvalue 0)
  (Variables|Default|SetHUD _returnvalue))

(event Custom|DestroyComponent
  (params (Target%20Component :type Actor%20Component%20Object%20Reference))
  ;[1 1 1] Destroy Component
  (Components|DestroyComponent Target%20Component))

(event Custom|Walk%20VFX
  ;[1 1 1] Walk VFX (Broken)
  (if (Variables|Default|GetwalkVFX)
    (bind _returnvalue (Niagara|SpawnSystematLocation "/Game/Design/VFX/NS_WalkingRubble.NS_WalkingRubble" (Transformation|GetWorldLocation (Variables|Character|GetMesh))))
    (Niagara|SetNiagaraVariable(LinearColor) _returnvalue "FloorColour" (Variables|Default|GetFloorColour))
    (Variables|Default|SetwalkVFX false)
    (Utilities|FlowControl|Delay 0.3)
    (Variables|Default|SetwalkVFX true)))

(event Custom|Init%20Cam
  ;[1 1 1] Init
)

(event Input|EnhancedActionEvents|EnhancedInputActionIA_2DMove
  (params (ActionValue :type Float%20%28double-precision%29) (ElapsedSeconds :type Float%20%28double-precision%29) (TriggeredSeconds :type Float%20%28double-precision%29) (InputAction :type Input%20Action%20Object%20Reference :default "/Game/Tech/Core/Input/Actions/IA_2DMove.IA_2DMove"))
  ;[1 1 1] Movement Handling
  ;;[1 1 1] 2D Move
  (:Triggered
    (Pawn|Input|AddMovementInput (Math|Vector|GetForwardVector (Variables|Default|GetForwardVec)) ActionValue false)
    (CallFunction|SetRotation(Velocity))
    (CallFunction|WalkVFX)))

(event Input|EnhancedActionEvents|EnhancedInputActionIA_Move
  (params (ActionValue :type Vector%202D%20Structure) (ElapsedSeconds :type Float%20%28double-precision%29) (TriggeredSeconds :type Float%20%28double-precision%29) (InputAction :type Input%20Action%20Object%20Reference :default "/Game/Tech/Core/Input/Actions/IA_Move.IA_Move"))
  ;[1 1 1] Movement Handling
  ;;[1 1 1] 3D Move
  (:Triggered
    (Pawn|Input|AddMovementInput (Math|Vector|GetRightVector (Variables|Default|GetForwardVec)) (.x ActionValue) false)
    (Pawn|Input|AddMovementInput (Math|Vector|GetForwardVector (Variables|Default|GetForwardVec)) (.y ActionValue) false)
    (CallFunction|SetRotation(Velocity))
    (CallFunction|WalkVFX)))

(event Input|EnhancedActionEvents|EnhancedInputActionIA_LaunchBuildMode
  (params (ActionValue :type Boolean) (ElapsedSeconds :type Float%20%28double-precision%29) (TriggeredSeconds :type Float%20%28double-precision%29) (InputAction :type Input%20Action%20Object%20Reference :default "/Game/Tech/BuildSystem/InputActions/IA_LaunchBuildMode.IA_LaunchBuildMode"))
  ;[1 1 1] Launch Build Mode
  (:Started
    (Default|LaunchBuildMode (Variables|Default|GetBPC_BuildComponent))))

(event Input|EnhancedActionEvents|EnhancedInputActionIA_Interact
  (params (ActionValue :type Boolean) (ElapsedSeconds :type Float%20%28double-precision%29) (TriggeredSeconds :type Float%20%28double-precision%29) (InputAction :type Input%20Action%20Object%20Reference :default "/Game/Tech/Core/Input/Actions/IA_Interact.IA_Interact"))
  (bind _returnvalue (Transformation|GetActorLocation))
  (bind _returnvalue_2 (Math|Conversions|ToVector(Float) 1e+02))
  ;[1 1 1] Interact
  (:Started
    (Rendering|Debug|DrawDebugBox _returnvalue _returnvalue_2 "(R=1.000000,G=0.000000,B=0.000000,A=1.000000)" "0, 0, 0" 0.1 3.0)
    (bind (_outactors _returnvalue_3) (Collision|BoxOverlapActors _returnvalue _returnvalue_2 (Utilities|Array|MakeArray "ObjectTypeQuery1" "ObjectTypeQuery2" "ObjectTypeQuery3") "/Game/Tech/Interactables/BP_InteractableMaster.BP_InteractableMaster_C" :!class /Script/Engine.KismetSystemLibrary))
    (if _returnvalue_3
      (for _array_element _outactors
        (Class|BPI|Interact(Message) _array_element 0 (Utilities|Array|Get(acopy) (Variables|/Game/Tech/Inventory/BPC_Inventory.BPC_Inventory_C|GetInventory (Variables|Default|GetBPC_Inventory)) (Variables|Default|GetSelectedInventorySlot)))))))

(event Input|EnhancedActionEvents|EnhancedInputActionIA_ConfimBuild
  (params (ActionValue :type Boolean) (ElapsedSeconds :type Float%20%28double-precision%29) (TriggeredSeconds :type Float%20%28double-precision%29) (InputAction :type Input%20Action%20Object%20Reference :default "/Game/Tech/BuildSystem/InputActions/IA_ConfimBuild.IA_ConfimBuild"))
  (bind _bpc_buildcomponent (Variables|Default|GetBPC_BuildComponent))
  ;[1 1 1] Confirm Build
  (:Started
    (if (and (Variables|/Game/Tech/BuildSystem/Blueprints/BPC_BuildComponent.BPC_BuildComponent_C|GetIsBuildModeOn? _bpc_buildcomponent) (Variables|/Game/Tech/BuildSystem/Blueprints/BPC_BuildComponent.BPC_BuildComponent_C|GetCanBuild? _bpc_buildcomponent))
      (Default|SpawnBuild (Variables|Default|GetBPC_BuildComponent)))))

(event Input|EnhancedActionEvents|EnhancedInputActionIA_InventoryScroll
  (params (ActionValue :type Float%20%28double-precision%29) (ElapsedSeconds :type Float%20%28double-precision%29) (TriggeredSeconds :type Float%20%28double-precision%29) (InputAction :type Input%20Action%20Object%20Reference :default "/Game/Tech/Core/Input/Actions/IA_InventoryScroll.IA_InventoryScroll"))
  ;[1 1 1] Select Inv Slot
  (:Triggered
    (bind _output_get (Variables|Default|SetSelectedInventorySlot (Math|Integer|Clamp(Integer) (+ (Math|Float|Truncate ActionValue) (Variables|Default|GetSelectedInventorySlot)) 0 (- (Variables|/Game/Tech/Inventory/BPC_Inventory.BPC_Inventory_C|GetMaxInventorySize (Variables|Default|GetBPC_Inventory)) 1))))
    (Default|CallSelectedSlotUpdated (Variables|Default|GetBPC_Inventory) _output_get)))

(event Input|EnhancedActionEvents|EnhancedInputActionIA_Pause
  (params (ActionValue :type Boolean) (ElapsedSeconds :type Float%20%28double-precision%29) (TriggeredSeconds :type Float%20%28double-precision%29) (InputAction :type Input%20Action%20Object%20Reference :default "/Game/Tech/Core/Input/Actions/IA_Pause.IA_Pause"))
  ;[1 1 1] Menu
  (:Started
    (bind _returnvalue (UserInterface|CreateWidget "/Game/Design/UI/UI_Options.UI_Options_C"))
    (UserInterface|Viewport|AddtoViewport _returnvalue 0)))

(event EventBeginPlay
  (CallFunction|Init))

(fn ConstructionScript)

(fn SetRotation(Velocity)
  (bind _charactermovement (Variables|Character|GetCharacterMovement))
  (bind _velocity (Variables|/Script/Engine.MovementComponent|GetVelocity _charactermovement))
  (bind _returnvalue (Math|Vector|Normalize _velocity))
  (bind _returnvalue_2 (Math|Conversions|RotationFromXVector _returnvalue))
  (Transformation|SetRelativeRotation (Variables|Character|GetMesh) (Math|Rotator|MakeRotator (+ (.roll _returnvalue_2) 9e+01) (.pitch _returnvalue_2) (- (.yaw _returnvalue_2) 9e+01)) false false))