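; Customer actor that requests a food item when interacted with and accepts it from the player's held item.
; SelectFood follows the hardcoded Fish row in DT_OvenData to its output item, stores it as DesiredFood and shows its texture on FoodBillboard.
; Later interactions compare item names, removing a match from its inventory and clearing the order.
; An unconnected random selection from DT_Items remains unused.
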(event Custom|Select%20food
  (bind _foodbillboard (Variables|Default|GetFoodBillboard))
  (bind _returnvalue (Utilities|GetDataTableRow "/Game/Tech/Static_Data/Food/DT_OvenData.DT_OvenData" "Fish")
    (:then
      (bind _returnvalue_2 (Utilities|GetDataTableRow (.DataTable (Utilities|Struct|BreakDataTableRowHandle (.OutputItem (Utilities|Struct|BreaksFood _returnvalue)))) (.RowName (Utilities|Struct|BreakDataTableRowHandle (.OutputItem (Utilities|Struct|BreaksFood _returnvalue)))))
        (:then
          ;[0.901 0.5591 0.3091] Select food
          (bind _output_get (Variables|Default|SetDesired%20Food _returnvalue_2))
          (Rendering|Components|Sprite|SetSprite _foodbillboard (.Texture (Utilities|Struct|BreaksItem _output_get)))
          (Components|Activation|SetActive _foodbillboard true false)
          (Variables|Default|SetGivenOrder true))
        (:RowNotFound
          (Development|PrintString "THIS DOES NOT EXIST"))))))

(event EventBeginPlay
  (Components|Activation|SetActive (Variables|Default|GetFoodBillboard) false false))

(event Collision|EventActorBeginOverlap
  (params (OtherActor :type Actor%20Object%20Reference)))

(event EventTick
  (params (DeltaSeconds :type Float%20%28single-precision%29)))

(event EventInteractionwithHeldItem
  (params (ItemInHand :type S%20Item%20Structure))
  (bind (_itemname _texture _amount_shouldbe1 _isstackable _maxstack _mesh _linkedgrowdata _linkedovendata _linkedpotdata _linkedchopdata _itemquality_ignore _owninginventory_ignore) (Utilities|Struct|BreaksItem ItemInHand))
  (bind _foodbillboard (Variables|Default|GetFoodBillboard))
  ;[0 1 0.0264] Interaction
  (if (Variables|Default|GetGivenOrder)
    (if (Utilities|Enum|Equal(Enum) _itemname (.ItemName (Utilities|Struct|BreaksItem (Variables|Default|GetDesired%20Food))))
      (Default|RemoveItem _owninginventory_ignore ItemInHand)
      (Development|PrintString "CORRECT  Item")
      (Rendering|Components|Sprite|SetSprite _foodbillboard 0)
      (Components|Activation|SetActive _foodbillboard false false)
      (Variables|Default|SetGivenOrder false)
      (else
        (Development|PrintString "Incorrect Item")))
    (else
      (CallFunction|SelectFood))))

(fn ConstructionScript
  (|CallParentFunction))