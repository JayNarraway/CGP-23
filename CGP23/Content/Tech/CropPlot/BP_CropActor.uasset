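; Crop plot actor where interacting harvests, plants from the held item or waters, falling back to advancing growth as a test hook.
; Data table rows link items to growables, whose stages advance only while watered.
; Growth mode either scales one mesh or swaps meshes per stage.
; At full growth, harvest mode either spawns a pickup or displays the produce for collection into the player's inventory, multiplied by yield.
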(event Custom|ResetGrowthStage
  (Variables|Default|SetCurrentGrowthStage 0))

(event Custom|SetGrowthStage
  (params (New%20Growth%20Stage :type Integer))
  (if (<= New%20Growth%20Stage (Variables|Default|GetGrowthStageLimit))
    (Variables|Default|SetCurrentGrowthStage New%20Growth%20Stage)))

(event Custom|CompleteGrowthBasedOnHarvestMode
  (bind _currentgrowable (Variables|Default|GetCurrentGrowable))
  (bind (_out_growable _out_result) (CallFunction|GetGrowableStructurefromGrowableRow _currentgrowable))
  (bind (_out_growable_2 _out_result_2) (CallFunction|GetGrowableStructurefromGrowableRow _currentgrowable))
  (switch Utilities|FlowControl|Switch|SwitchonENM_HarvestModes (Variables|Default|GetHarvestMode)
    (:NewEnumerator0
      (if _out_result
        (CallFunction|SpawnGrowablesLinkedItem _out_growable)))
    (:NewEnumerator1
      (if _out_result_2
        (CallFunction|PresentGrowablesLinkedItem _out_growable_2)))))

(event Custom|SetWateredState
  (params (New%20Watered%20State :type Boolean))
  (Variables|Default|SetIsWatered New%20Watered%20State))

(event Custom|SpawnGrowablesLinkedItem
  (params (Growable%20Input :type S%20Growable%20Structure))
  (bind _grownitem (Utilities|Struct|BreaksGrowable Growable%20Input))
  (bind (_datatable _rowname) (Utilities|Struct|BreakDataTableRowHandle _grownitem))
  ;[1 1 1] immediately ejects item, Used for walk into to pick up item
  (Class|DataTableFunctionLibrary|DoesDataTableRowExist _datatable _rowname)
  (if (!= _rowname "EMPTY")
    ;[1 1 1] need to spawn item but the object and class requires setting up for each instance spawning, need a premade thing to spawn without touching it
    (bind _returnvalue (Game|SpawnActorfromClass "/Game/Blueprints/Inventory/BP_BaseItem.BP_BaseItem_C" (Math|Transform|MakeTransform (.location (Transformation|GetWorldTransform (Variables|Default|GetDropPoint))) "0, 0, 0" (Class|KismetMathLibrary|VectorOne)) "Undefined" "MultiplyWithRoot" 0 (Utilities|Struct|MakeDataTableRowHandle _datatable _rowname) 0))
    (Components|StaticMesh|SetStaticMesh (Variables|/Game/Blueprints/Inventory/BP_BaseItem.BP_BaseItem_C|GetItemMesh _returnvalue) (.Mesh (Utilities|Struct|BreaksItem (CallFunction|GetItemfromGrowable Growable%20Input))))
    (Variables|Default|SetCanHarvest false)))

(event Custom|PresentGrowablesLinkedItem
  (params (Growable%20Input :type S%20Growable%20Structure))
  (bind _grownitem (Utilities|Struct|BreaksGrowable Growable%20Input))
  (bind (_datatable _rowname) (Utilities|Struct|BreakDataTableRowHandle _grownitem))
  ;[1 1 1] presents item in a hold, Used for interact to harvest item and logic to actually present it
  (Variables|Default|SetCanHarvest true)
  (Class|DataTableFunctionLibrary|DoesDataTableRowExist _datatable _rowname)
  (if (!= _rowname "EMPTY")
    (Components|StaticMesh|SetStaticMesh (Variables|Default|GetPendingItem) (.Mesh (Utilities|Struct|BreaksItem (CallFunction|GetItemfromGrowable Growable%20Input))))))

(event Custom|CheckForCompletedGrowth
  (if (Math|Boolean|ANDBoolean (not (Variables|Default|GetCanHarvest)) (>= (Variables|Default|GetCurrentGrowthStage) (Variables|Default|GetGrowthStageLimit)) (Variables|Default|GetIsWatered))
    (CallFunction|CompleteGrowthBasedonHarvestMode)))

(event Custom|IncrementGrowthStage
  (bind _currentgrowable (Variables|Default|GetCurrentGrowable))
  (bind (_out_growable _out_result) (CallFunction|GetGrowableStructurefromGrowableRow _currentgrowable))
  (if (< (Variables|Default|GetCurrentGrowthStage) (Variables|Default|GetGrowthStageLimit))
    (if (Variables|Default|GetIsWatered)
      (bind _result (Math|Integer|IncrementInt (Variables|Default|GetCurrentGrowthStage))
        (:%20%20
          (Variables|Default|SetCurrentGrowthStage _result)
          (CallFunction|UpdateGrowableVisual)
          (CallFunction|CheckforCompletedGrowth))))
    (elif (and _out_result (Utilities|Enum|NotEqual(Enum) (.PlantName (Utilities|Struct|BreaksGrowable _out_growable)) (Variables|Default|GetEmptyGrowable)))
      (CallFunction|UpdateGrowableVisual)
      (CallFunction|CheckforCompletedGrowth))))

(event Custom|SetYieldMultiplier
  (params (New%20Multiplier :type Integer))
  (Variables|Default|SetYieldMultiplier New%20Multiplier))

(event Custom|CompileGrowthProperties
  (switch Utilities|FlowControl|Switch|SwitchonENM_GrowthModes (Variables|Default|GetGrowthMode)
    (:NewEnumerator0
      (if (not (Utilities|IsValid (Utilities|Array|Get(acopy) (Variables|Default|GetGrowthGraphics))))
        (Variables|Default|SetGrowthGraphics (Utilities|Array|MakeArray 0))))
    (:NewEnumerator1
      (CallFunction|RecalculateMeshSlotsCount))))

(event Custom|SetGrowthStageLimit
  (params (New%20Growth%20Stage%20Limit :type Integer))
  (Variables|Default|SetGrowthStageLimit New%20Growth%20Stage%20Limit))

(event Custom|SetCurrentGrowable
  (params (Growable%20Input :type S%20Growable%20Structure))
  ;[1 1 1] Sets the current growable on the crop to the growable passed in
  (CallFunction|ResetGrowthStage)
  (CallFunction|SetGrowthStageLimit (Math|Float|Truncate (.GrowTime (Utilities|Struct|BreaksGrowable Growable%20Input))))
  (bind _out_row_reference (CallFunction|GetGrowableRowfromGrowableStructure Growable%20Input))
  (Variables|Default|SetCurrentGrowable _out_row_reference))

(event Custom|UpdateGrowableVisual
  ;[1 1 1] Call to update how the growing element looks. Do this after updating the data for the growing item's progression
  (switch Utilities|FlowControl|Switch|SwitchonENM_GrowthModes (Variables|Default|GetGrowthMode)
    (:NewEnumerator0
      (CallFunction|UpdateGrowableMeshScale))
    (:NewEnumerator1
      (CallFunction|UpdateGrowableMeshType))))

(event Custom|UpdateGrowableMeshScale
  (bind _currentgrowablemesh (Variables|Default|GetCurrentGrowableMesh))
  (bind _currentgrowable (Variables|Default|GetCurrentGrowable))
  (bind _out_growable (CallFunction|GetGrowableStructurefromGrowableRow _currentgrowable))
  (bind _mesh (Utilities|Struct|BreaksGrowable _out_growable))
  ;[1 1 1] is there a mesh to update
  (if (Utilities|IsValid (Variables|/Script/Engine.StaticMeshComponent|GetStaticMesh (Variables|Default|GetCurrentGrowableMesh)))
    ;[1 1 1] then update it's scale
    (Transformation|SetRelativeScale3D _currentgrowablemesh (* (/ (Variables|Default|GetCurrentGrowthStage) (Variables|Default|GetGrowthStageLimit)) (Class|KismetMathLibrary|VectorOne)) :!label _label)
    (else
      ;[1 1 1] do we have one in the array?
      (if (Utilities|IsValid (Utilities|Array|Get(acopy) (Variables|Default|GetGrowthGraphics)))
        (bind _returnvalue (Components|StaticMesh|SetStaticMesh _currentgrowablemesh (Utilities|Array|Get(acopy) (Variables|Default|GetGrowthGraphics)) :!label _label_2))
        (if _returnvalue
          (goto _label))
        (else
          ;[1 1 1] can we use a mesh at all?
          (if (Utilities|IsValid _mesh)
            (Variables|Default|SetGrowthGraphics (Utilities|Array|MakeArray _mesh))
            (goto _label_2)))))))

(event Custom|UpdateGrowableMeshType
  (Components|StaticMesh|SetStaticMesh (Variables|Default|GetCurrentGrowableMesh) (Utilities|Array|Get(acopy) (Variables|Default|GetGrowthGraphics) (Variables|Default|GetCurrentGrowthStage))))

(event EventInteract
  (params (HitComponent :type Primitive%20Component%20Object%20Reference) (ItemInHand :type S%20Item%20Structure))
  (bind _out_result (CallFunction|CheckforCollection))
  ;[1 1 1] Condition for collecting
  (if _out_result
    (CallFunction|DoCollection (Variables|Default|GetCurrentGrowable) (Variables|Default|GetYieldMultiplier))
    (else
      (bind _out_result_2 (CallFunction|CheckforPlanting ItemInHand))
      ;[1 1 1] Condition for planting
      (if _out_result_2
        (CallFunction|SetCurrentGrowable (CallFunction|GetGrowablefromItem ItemInHand))
        (Default|RemoveItem (.OwningInventory-IGNORE (Utilities|Struct|BreaksItem ItemInHand)) ItemInHand)
        (CallFunction|UpdateGrowableVisual)
        (else
          (bind _out_result_3 (CallFunction|CheckforWatering ItemInHand))
          ;[1 1 1] Condition for watering
          (if _out_result_3
            (CallFunction|SetWateredState true)
            (else
              ;[1 1 1] This needs to be called to test the system, hence why it's chucked on the end here
              (CallFunction|IncrementGrowthStage))))))))

(fn ConstructionScript
  (|CallParentFunction))

(fn GetItemfromGrowable
  (params (Growable%20in :type S%20Growable%20Structure))
  (bind _grownitem (Utilities|Struct|BreaksGrowable Growable%20in))
  (bind (_datatable _rowname) (Utilities|Struct|BreakDataTableRowHandle _grownitem))
  (bind _returnvalue (Class|DataTableFunctionLibrary|DoesDataTableRowExist _datatable _rowname))
  (if _returnvalue
    (bind _returnvalue_2 (Utilities|GetDataTableRow (LocalVariables|GetTableReference) _rowname)
      (:then
        (if (Utilities|Enum|NotEqual(Enum) (.ItemName (Utilities|Struct|BreaksItem _returnvalue_2)) (Variables|Default|GetEmptyItem))
          (return _returnvalue_2))))))

(fn GetGrowablefromItem
  (params (Item%20in :type S%20Item%20Structure))
  (bind _linkedgrowdata (Utilities|Struct|BreaksItem Item%20in))
  (bind (_datatable _rowname) (Utilities|Struct|BreakDataTableRowHandle _linkedgrowdata))
  (bind _returnvalue (Class|DataTableFunctionLibrary|DoesDataTableRowExist _datatable _rowname))
  (if _returnvalue
    (bind _returnvalue_2 (Utilities|GetDataTableRow (LocalVariables|GetTableReference) _rowname)
      (:then
        (if (Utilities|Enum|NotEqual(Enum) (.PlantName (Utilities|Struct|BreaksGrowable _returnvalue_2)) (Variables|Default|GetEmptyGrowable))
          (return _returnvalue_2))))))

(fn CheckforCollection
  (return (Math|Boolean|ANDBoolean (Variables|Default|GetCanHarvest) (Utilities|Enum|Equal(Enum) (Variables|Default|GetHarvestMode) "NewEnumerator1") (not (Utilities|Text|TextIsEmpty (.PlantName (Utilities|Struct|BreaksGrowable (.Out%20Growable (CallFunction|GetGrowableStructurefromGrowableRow (Variables|Default|GetCurrentGrowable))))))))))

(fn CheckforPlanting
  (params (In%20Item :type S%20Item%20Structure))
  (bind (_itemname _linkedgrowdata) (Utilities|Struct|BreaksItem In%20Item))
  (return (Math|Boolean|ANDBoolean (Utilities|Enum|NotEqual(Enum) _itemname (Variables|Default|GetEmptyItem)) (Utilities|Enum|Equal(Enum) (Variables|Default|GetEmptyGrowable) (.PlantName (Utilities|Struct|BreaksGrowable (.Out%20Growable (CallFunction|GetGrowableStructurefromGrowableRow (Variables|Default|GetCurrentGrowable)))))) (!= "EMPTY" (.RowName (Utilities|Struct|BreakDataTableRowHandle _linkedgrowdata))))))

(fn CheckforWatering
  (params (In%20Item :type S%20Item%20Structure))
  (bind _wateringitem (Variables|Default|GetWateringItem))
  (bind (_datatable _rowname) (Utilities|Struct|BreakDataTableRowHandle _wateringitem))
  (bind _returnvalue (Utilities|GetDataTableRow _datatable _rowname)
    (:then
      (return (Math|Boolean|ANDBoolean (Utilities|Enum|Equal(Enum) (Utilities|String|ToString(Text) (.ItemName (Utilities|Struct|BreaksItem _returnvalue))) (Utilities|String|ToString(Text) (.ItemName (Utilities|Struct|BreaksItem In%20Item)))) (not (Utilities|Enum|Equal(Enum) (Variables|Default|GetEmptyItem) (.PlantName (Utilities|Struct|BreaksGrowable (.Out%20Growable (CallFunction|GetGrowableStructurefromGrowableRow (Variables|Default|GetCurrentGrowable))))))) (not (Variables|Default|GetIsWatered)))))))

(fn RecalculateMeshSlotsCount
  (bind _array_element (Utilities|Array|ForEachLoopwithBreak (Variables|Default|GetGrowthGraphics))
    (:LoopBody
      (if (Utilities|IsValid _array_element)
        (LocalVariables|SetHasAnUnemptyGraphic true)))
    (:Completed
      (if (not (LocalVariables|GetHasAnUnemptyGraphic))
        (Variables|Default|SetGrowthGraphics (Utilities|Array|MakeArray))
        (for _index (range 0 (- (Variables|Default|GetGrowthStageLimit) (LocalVariables|GetArrayIndexOffset)))
          (Utilities|Array|AppendArray (Variables|Default|GetGrowthGraphics) (Utilities|Array|MakeArray 0)))))))

(fn GetCorrectMeshfromGrowable
  (params (In%20Current :type Integer) (In%20Limit :type Integer) (In%20Meshes%20%28Array%29 :type Array%20of%20Static%20Mesh%20Object%20References))
  (bind _output (Utilities|Array|Get(acopy) In%20Meshes%20%28Array%29))
  (bind _filteredarray (LocalVariables|GetFilteredArray))
  (bind _filteredarray_2 (LocalVariables|GetFilteredArray))
  (bind _returnvalue (Utilities|Array|Length _filteredarray_2))
  (bind _output_2 (Utilities|Array|Get(acopy) _filteredarray In%20Current))
  (switch Utilities|FlowControl|Switch|SwitchonENM_GrowthModes (Variables|Default|GetGrowthMode)
    (:NewEnumerator0
      ;[1 1 1] Get the only (first) mesh there is and if exists, return it
      (if (Utilities|IsValid _output)
        (return _output true)
        (else
          (return 0 false))))
    (:NewEnumerator1
      (switch Utilities|FlowControl|Switch|SwitchonENM_MeshAssignmentModes (Variables|Default|GetMeshAssignmentMode)
        (:NewEnumerator0
          ;[1 1 1] Get the mesh using the current growth stage as the index to look at and return if success
          (for _array_element In%20Meshes%20%28Array%29
            (if (Utilities|IsValid _array_element)
              (Utilities|Array|AppendArray (LocalVariables|GetFilteredArray) (Utilities|Array|MakeArray _array_element))))
          (if (Utilities|IsValid _output_2)
            (return _output_2 true)
            (else
              (return 0 false))))
        (:NewEnumerator1
          (for _array_element_2 In%20Meshes%20%28Array%29
            (if (Utilities|IsValid _array_element_2)
              (Utilities|Array|AppendArray (LocalVariables|GetFilteredArray) (Utilities|Array|MakeArray _array_element_2))))
          ;[1 1 1] Percent = (current / max) * 100
          (LocalVariables|SetCurrentPercentage (* (/ In%20Current In%20Limit) 1e+02))
          ;[1 1 1] Runs on index first, last, and all inbetween
          (for _index (range 0 (- _returnvalue 1))
            (if (and (< (* _index (/ 100 _returnvalue)) (LocalVariables|GetCurrentPercentage)) (<= (LocalVariables|GetCurrentPercentage) (* (+ _index 1) (/ 100 _returnvalue))))
              (return (Utilities|Array|Get(acopy) (LocalVariables|GetFilteredArray) _index) true)
              (elif (== (LocalVariables|GetCurrentPercentage) (* (+ _index 1) (/ 100 _returnvalue)))
                (return (Utilities|Array|Get(acopy) (LocalVariables|GetFilteredArray) _index) true))))
          ;[1 1 1] Loop fail
          (return 0 false))))))

(fn GetGrowableStructurefromGrowableRow
  (params (In%20Growable%20Row :type Data%20Table%20Row%20Handle%20Structure))
  (bind _returnvalue (Utilities|GetDataTableRow "/Game/Static_Data/Plants/DT_GrowData.DT_GrowData" (.RowName (Utilities|Struct|BreakDataTableRowHandle In%20Growable%20Row)))
    (:then
      (return _returnvalue true))
    (:RowNotFound
      (return "" false))))

(fn GetItemStructurefromItemRow
  (params (In%20Item%20Row :type Data%20Table%20Row%20Handle%20Structure))
  (bind (_datatable _rowname) (Utilities|Struct|BreakDataTableRowHandle In%20Item%20Row))
  (bind _returnvalue (Utilities|GetDataTableRow _datatable _rowname)
    (:then
      (return _returnvalue true))
    (:RowNotFound
      (return "" false))))

(fn GetGrowableRowfromGrowableStructure
  (params (In%20growable :type S%20Growable%20Structure))
  (bind _tablereference (LocalVariables|GetTableReference))
  (bind _outrownames (DataTable|GetDataTableRowNames _tablereference))
  (for _array_element _outrownames
    (if (Utilities|Enum|Equal(Enum) (Utilities|String|ToString(Name) _array_element) (Utilities|String|ToString(Text) (.PlantName (Utilities|Struct|BreaksGrowable In%20growable))))
      (return (Utilities|Struct|MakeDataTableRowHandle _tablereference _array_element) true)))
  (return "" false))

(fn DoCollection
  (params (In%20Growable :type Data%20Table%20Row%20Handle%20Structure) (In%20Multiplier :type Integer))
  (bind _returnvalue (Actor|GetActorOfClass "/Game/Player/_PLAYER._PLAYER_C"))
  (bind _as_player (Utilities|Casting|CastTo_PLAYER _returnvalue))
  (for _index (range 1 In%20Multiplier)
    (Default|AddItemtoInventory (Variables|/Game/Player/_PLAYER._PLAYER_C|GetBPC_Inventory _as_player) (CallFunction|GetItemfromGrowable (.Out%20Growable (CallFunction|GetGrowableStructurefromGrowableRow In%20Growable)))))
  (Variables|Default|SetCanHarvest false)
  (Components|StaticMesh|SetStaticMesh (Variables|Default|GetPendingItem) 0))