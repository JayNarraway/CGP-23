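; Inventory component for the quest system that holds an item-to-value map and reports item additions as objective progress.
; AddToInventory writes the item's existing map value back without adding Quantity, then calls OnObjectiveIDCalled on the player character with the item name as objective ID and Quantity as value.
; QueryInventory returns the stored value for an item.
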(event EventBeginPlay)

(event EventTick
  (params (DeltaSeconds :type Float%20%28single-precision%29)))

(fn AddtoInventory
  (params (Item :type Name) (Quantity :type Integer))
  (Utilities|Map|Add (Variables|Default|GetContent) Item (.Value (Utilities|Map|Find (Variables|Default|GetContent) Item)))
  (bind _as_player (Utilities|Casting|CastTo_PLAYER (Game|GetPlayerCharacter 0)))
  (Default|CallOnObjectiveIDCalled _as_player (Utilities|String|ToString(Name) Item) Quantity))

(fn QueryInventory
  (params (Item :type Name))
  (return (.Value (Utilities|Map|Find (Variables|Default|GetContent) Item))))