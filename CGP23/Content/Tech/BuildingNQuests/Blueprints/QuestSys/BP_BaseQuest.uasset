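; Base quest Blueprint that tracks one quest's progress through the stages and objectives defined in DT_QuestData.
; BeginPlay loads the current stage, listens to the player's objective-ID event and seeds one objective type from an inventory query.
; Objective events update a progress map, showing a notification widget when an objective reaches its quantity.
; Finished stages load the next, and the last marks completion, turning in through BPC_QuestLog if AutoComplete is set.
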(event EventBeginPlay
  (CallFunction|GetQuestDetails)
  (bind _as_player (Utilities|Casting|CastTo_PLAYER (Game|GetPlayerCharacter 0)))
  (bind _output_get (Variables|Default|SetPLayerRef _as_player))
  (EventDispatchers|BindEventtoOnObjectiveIDCalled _output_get (EventDispatchers|CreateEvent :!event OnObjectiveIDHeard))
  (for _array_element (.Objectives (Utilities|Struct|BreakS_StageDetails (Variables|Default|GetCurrentStageDetails)))
    ;[1 1 1] Why would this not wokr
    (Development|PrintString (Utilities|String|ToString(Name) (Utilities|Name|EnumtoName (.Type (Utilities|Struct|BreakS_ObjectiveDetails _array_element)))))
    (if (Utilities|Enum|Equal(Enum) (.Type (Utilities|Struct|BreakS_ObjectiveDetails _array_element)) "NewEnumerator3")
      (bind _value (Default|QueryInventory (Variables|/Game/Player/_PLAYER._PLAYER_C|GetBPC_InventoryQuestChecker (Variables|Default|GetPLayerRef)) (Utilities|String|StringToName (.ObjectiveID (Utilities|Struct|BreakS_ObjectiveDetails _array_element)))))
      (CallFunction|OnObjectiveIDHeard (.ObjectiveID (Utilities|Struct|BreakS_ObjectiveDetails _array_element)) _value)))
  (bind _return (CallFunction|AreObjectivesComplete))
  (Variables|Default|SetIs%20Completed? _return))

(fn ConstructionScript)

(fn OnObjectiveIDHeard
  (params (ObjectiveID :type String) (Value :type Integer))
  (bind _currentobjectiveprogress (Variables|Default|GetCurrentObjectiveProgress))
  (bind (_value _returnvalue) (Utilities|Map|Find _currentobjectiveprogress ObjectiveID))
  (if (> (Class|KismetMathLibrary|SignOfInteger Value) 0)
    (if _returnvalue
      (if (< _value (.Quantity (Utilities|Struct|BreakS_ObjectiveDetails (CallFunction|GetObjectiveDatabyID ObjectiveID))))
        (Utilities|Map|Add (Variables|Default|GetCurrentObjectiveProgress) ObjectiveID (+ _value Value))
        (CallFunction|IsObjectiveComplete ObjectiveID)
        (Default|CallOnObjectiveHeard)
        (return))
      (else
        (return)))
    (else
      (Utilities|Map|Add (Variables|Default|GetCurrentObjectiveProgress) ObjectiveID (+ (.Value (Utilities|Map|Find (Variables|Default|GetCurrentObjectiveProgress) ObjectiveID)) Value))
      (return))))

(fn GetQuestDetails
  ;[1 1 1] Basically anytime you want to access the quest data just pull this up
  (bind _returnvalue (Utilities|GetDataTableRow "/Game/Tech/BuildingNQuests/Blueprints/QuestSys/DT_QuestData.DT_QuestData" (Variables|Default|GetQuestID))
    (:then
      ;[1 1 1] For referencing elsewhere in the blueprint
      (bind _output_get (Variables|Default|SetQuestDetails _returnvalue))
      (bind _output_get_2 (Variables|Default|SetCurrentStageDetails (Utilities|Array|Get(acopy) (.Stages (Utilities|Struct|BreakS_QuestDetailsStruct _output_get)) (Variables|Default|GetCurrentStage))))
      (Utilities|Map|Clear (Variables|Default|GetCurrentObjectiveProgress))
      (for _array_element (Utilities|Struct|BreakS_StageDetails _output_get_2)
        (Utilities|Map|Add (Variables|Default|GetCurrentObjectiveProgress) (Utilities|Struct|BreakS_ObjectiveDetails _array_element) 0)))))

(fn GetObjectiveDatabyID
  (params (ObjectiveID :type String))
  (for _array_element (.Objectives (Utilities|Struct|BreakS_StageDetails (Variables|Default|GetCurrentStageDetails)))
    (if (Utilities|Enum|Equal(Enum) (.ObjectiveID (Utilities|Struct|BreakS_ObjectiveDetails _array_element)) ObjectiveID)
      (return _array_element))))

(fn IsObjectiveComplete
  (params (ObjectiveID :type String))
  (bind _array_element (CallFunction|GetObjectiveDatabyID ObjectiveID))
  (bind (_description _quantity) (Utilities|Struct|BreakS_ObjectiveDetails _array_element))
  ;[0.1107 0.9203 1] Just Gets all the values and displays it onto the viewport
  (if (>= (.Value (Utilities|Map|Find (Variables|Default|GetCurrentObjectiveProgress) ObjectiveID)) _quantity)
    (bind _returnvalue (UserInterface|CreateWidget "/Game/Tech/BuildingNQuests/Blueprints/QuestSys/QuestUI/W_QuestNotif.W_QuestNotif_C" 0 _description))
    (UserInterface|Viewport|AddtoViewport _returnvalue 0)
    ;[1 1 1] Comment
    (bind _return (CallFunction|AreObjectivesComplete))
    ;[1 1 1] Moves to the next stage
    (if _return
      (bind _result (Math|Integer|IncrementInt (Variables|Default|GetCurrentStage))
        (:%20%20
          ;;[1 1 1] If there are no more stages mark completed if there are then get more details
          (if (Utilities|Array|IsValidIndex (.stages (Variables|Default|GetQuestDetails)) _result)
            (CallFunction|GetQuestDetails)
            (else
              (Variables|Default|SetIs%20Completed? true)
              (if (.autocomplete (Variables|Default|GetQuestDetails))
                (Default|TurninQuest (Actor|GetComponentbyClass (Game|GetPlayerCharacter 0) "/Game/Tech/BuildingNQuests/Blueprints/QuestSys/BPC_QuestLog.BPC_QuestLog_C") (Variables|Default|GetQuestID))))))))))

(fn AreObjectivesComplete
  (for _array_element (.Objectives (Utilities|Struct|BreakS_StageDetails (Variables|Default|GetCurrentStageDetails)))
    (if (not (>= (.Value (Utilities|Map|Find (Variables|Default|GetCurrentObjectiveProgress) (.ObjectiveID (Utilities|Struct|BreakS_ObjectiveDetails _array_element)))) (.Quantity (Utilities|Struct|BreakS_ObjectiveDetails (CallFunction|GetObjectiveDatabyID (.ObjectiveID (Utilities|Struct|BreakS_ObjectiveDetails _array_element)))))))
      (bind _output_get (LocalVariables|SetLocal_AllComplete false))
      (return _output_get)))
  (return (LocalVariables|GetLocal_AllComplete)))