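; Quest log component that adds, tracks, queries and turns in quests.
; Each added quest records its ID as active and spawns a BP_BaseQuest actor, which is later looked up by ID.
; Turn-in only prints the stage's XP as a reward placeholder, then deactivates the quest, flags it turned in and calls OnQuestCompleted.
; Tracking creates a W_QuestTracker widget once and updates it thereafter.
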(event EventBeginPlay)

(event EventTick
  (params (DeltaSeconds :type Float%20%28single-precision%29)))

(fn AddNewQuest
  (params (QuestID :type Name))
  ;[1 1 1] Avoids Duplicates
  (Utilities|Array|AddUnique (Variables|Default|GetCurrentActiveQuests) QuestID)
  (bind _returnvalue (Game|SpawnActorfromClass "/Game/Tech/BuildingNQuests/Blueprints/QuestSys/BP_BaseQuest.BP_BaseQuest_C" (Math|Transform|MakeTransform "0, 0, 0" "0, 0, 0" "1.000000,1.000000,1.000000") "Undefined" "MultiplyWithRoot" 0 QuestID 0))
  (Utilities|Array|Add (Variables|Default|GetCurrentQuests) _returnvalue)
  (return _returnvalue))

(fn CompleteQuest
  (params (QuestID :type Name))
  (Utilities|Array|AddUnique (Variables|Default|GetCurrentActiveQuests) QuestID)
  (Utilities|Array|RemoveItem (Variables|Default|GetCurrentActiveQuests) QuestID)
  (bind _array_element (CallFunction|GetQuestActor QuestID))
  (Variables|/Game/Tech/BuildingNQuests/Blueprints/QuestSys/BP_BaseQuest.BP_BaseQuest_C|SetIsTurnedin _array_element true)
  (Default|CallOnQuestCompleted _array_element))

(fn QueryActiveQuest
  (params (QuestID :type Name))
  ;[1 1 1] Pure Function (Only Passes Info)
  (return (Utilities|Array|ContainsItem (Variables|Default|GetCurrentActiveQuests) QuestID)))

(fn TrackQuest
  (params (QuestActorRef :type BP%20Base%20Quest%20Object%20Reference))
  ;[1 1 1] WHERE IS THE TRACKING
  (bind _trackerref (Variables|Default|GetTrackerRef)
    (:then
      (Default|Update _trackerref QuestActorRef))
    (:else
      (bind _returnvalue (UserInterface|CreateWidget "/Game/Tech/BuildingNQuests/Blueprints/QuestSys/QuestUI/W_QuestTracker.W_QuestTracker_C" 0 QuestActorRef))
      (bind _output_get (Variables|Default|SetTrackerRef _returnvalue))
      (UserInterface|Viewport|AddtoViewport _output_get -1))))

(fn GetQuestActor
  (params (QuestID :type Name))
  (for _array_element (Variables|Default|GetCurrentQuests)
    (if (== (Variables|/Game/Tech/BuildingNQuests/Blueprints/QuestSys/BP_BaseQuest.BP_BaseQuest_C|GetQuestID _array_element) QuestID)
      (return _array_element))))

(fn TurninQuest
  (params (QuestID :type Name))
  (Utilities|FlowControl|Sequence
    (:then_0
      ;[1 1 1] Gets the rewards
      (bind _array_element (CallFunction|GetQuestActor QuestID))
      ;;[1 1 1] Add Jay's Currency System here for rewards
      ;; If its giving additional Item rewards then that too (Link to Inventory)
      (Development|PrintString (Utilities|String|ToString(Text) (Utilities|Text|FormatText "XP= {a}" (.XPReward (Utilities|Struct|BreakS_StageDetails (Variables|/Game/Tech/BuildingNQuests/Blueprints/QuestSys/BP_BaseQuest.BP_BaseQuest_C|GetCurrentStageDetails _array_element)))))))
    (:then_1
      (CallFunction|CompleteQuest QuestID))))

(fn QueryCompltedQuests
  (params (QuestID :type Name))
  (bind _completedquests (Variables|Default|GetCompletedQuests))
  (bind _returnvalue (Utilities|Array|ContainsItem _completedquests QuestID))
  ;[1 1 1] Pure Function (Only Passes Info)
  (bind _array_element (CallFunction|GetQuestActor QuestID))
  (Utilities|IsValid _array_element
    (:Is%20Valid
      (return _returnvalue (Variables|/Game/Tech/BuildingNQuests/Blueprints/QuestSys/BP_BaseQuest.BP_BaseQuest_C|GetIsTurnedin _array_element)))
    (:Is%20Not%20Valid
      (return _returnvalue true))))