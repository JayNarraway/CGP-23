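; BP_QuestSaveData stores and restores the player's quest log state.
; Saving copies the active and completed quest lists from the quest log and records each quest's objective progress and stage in a map keyed by QuestID.
; Loading re-adds each active quest through the log's AddNewQuest, applies its saved stage and progress, then restores both lists.
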(fn SaveQuestDetails
  (params (Quest :type BP%20Base%20Quest%20Object%20Reference))
  (Utilities|Map|Add (Variables|Default|GetQuestProgress) (Variables|/Game/Tech/BuildingNQuests/Blueprints/QuestSys/BP_BaseQuest.BP_BaseQuest_C|GetQuestID Quest) (Utilities|Struct|MakeS_QuestSaveDataStruct (Variables|/Game/Tech/BuildingNQuests/Blueprints/QuestSys/BP_BaseQuest.BP_BaseQuest_C|GetCurrentObjectiveProgress Quest) (Variables|/Game/Tech/BuildingNQuests/Blueprints/QuestSys/BP_BaseQuest.BP_BaseQuest_C|GetCurrentStage Quest))))

(fn LoadQuests
  (params (QuestLogRef :type BPC%20Quest%20Log%20Object%20Reference))
  (for _array_element (Variables|Default|GetCurrentActiveQuests)
    (bind _returnvalue (Default|AddNewQuest QuestLogRef _array_element))
    (Variables|/Game/Tech/BuildingNQuests/Blueprints/QuestSys/BP_BaseQuest.BP_BaseQuest_C|SetCurrentStage _returnvalue (.CurrentStage (Utilities|Struct|BreakS_QuestSaveDataStruct (.Value (Utilities|Map|Find (Variables|Default|GetQuestProgress) _array_element)))))
    (Variables|/Game/Tech/BuildingNQuests/Blueprints/QuestSys/BP_BaseQuest.BP_BaseQuest_C|SetCurrentObjectiveProgress _returnvalue (.Progress (Utilities|Struct|BreakS_QuestSaveDataStruct (.Value (Utilities|Map|Find (Variables|Default|GetQuestProgress) _array_element))))))
  (Variables|/Game/Tech/BuildingNQuests/Blueprints/QuestSys/BPC_QuestLog.BPC_QuestLog_C|SetCurrentActiveQuests QuestLogRef (Variables|Default|GetCurrentActiveQuests))
  (Variables|/Game/Tech/BuildingNQuests/Blueprints/QuestSys/BPC_QuestLog.BPC_QuestLog_C|SetCompletedQuests QuestLogRef (Variables|Default|GetCompleteQuests)))

(fn SaveQuestLog
  (params (QuestLogRef :type BPC%20Quest%20Log%20Object%20Reference))
  (Variables|Default|SetCurrentActiveQuests (Variables|/Game/Tech/BuildingNQuests/Blueprints/QuestSys/BPC_QuestLog.BPC_QuestLog_C|GetCurrentActiveQuests QuestLogRef))
  (Variables|Default|SetCompleteQuests (Variables|/Game/Tech/BuildingNQuests/Blueprints/QuestSys/BPC_QuestLog.BPC_QuestLog_C|GetCompletedQuests QuestLogRef)))