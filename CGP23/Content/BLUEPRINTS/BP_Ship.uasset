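; BP_Ship is a repairable ship that the player restores in Ladder, Mast and Flag stages by supplying inventory items.
; Interact moves matching items, named through data table rows, from the player's inventory component into the current requirements, shown on a widget component.
; When all requirements are met, NextStage applies the finished material to that part and loads the next list.
; Flag is the final stage; ShipRepaired is an empty stub.
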(event Custom|GetPlayerRef
  (bind _as_player (Utilities|Casting|CastTo_PLAYER (Game|GetPlayerCharacter 0)))
  (Variables|Default|SetAs%20PLAYER _as_player))

(event Custom|SetWidgetRef
  (bind _returnvalue (UserInterface|CreateWidget "/Game/UI/UI_ShipRequirements.UI_ShipRequirements_C"))
  (bind _output_get (Variables|Default|SetRequirementsUI _returnvalue))
  (UserInterface|SetWidget (Variables|Default|GetWidget) _output_get))

(event EventInteract
  (params (HitComponent :type Primitive%20Component%20Object%20Reference))
  (CallFunction|CheckPlayerInventory (Variables|Default|GetCurrentRequirements))
  (CallFunction|UpdateUI)
  (CallFunction|CheckifReqsMet))

(event EventBeginPlay
  (bind _currentrequirements (Variables|Default|GetCurrentRequirements))
  (CallFunction|GetPlayerRef)
  (CallFunction|SetWidgetRef)
  (Utilities|Array|Clear _currentrequirements)
  (for _array_element (Variables|STATIC_DATA|GetLadderReqs)
    (Utilities|Array|Add _currentrequirements _array_element))
  (CallFunction|UpdateUI))

(fn ConstructionScript)

(fn NextStage
  (params (CurrentStage :type eShipStage%20Enum :default "NewEnumerator4"))
  (bind _currentrequirements (Variables|Default|GetCurrentRequirements))
  (bind _currentrequirements_2 (Variables|Default|GetCurrentRequirements))
  (switch Utilities|FlowControl|Switch|SwitchoneShipStage CurrentStage
    (:NewEnumerator4
      (Rendering|Material|SetMaterial (Variables|Default|GetLadder) 0 "/Game/Assets/Materials/M_ShipWood.M_ShipWood")
      (Variables|Default|SetCurrentWorkingStage "NewEnumerator5")
      (Utilities|Array|Clear _currentrequirements)
      (for _array_element (Variables|STATICDATA|GetMastReqs)
        (Utilities|Array|Add _currentrequirements _array_element)))
    (:NewEnumerator5
      (Rendering|Material|SetMaterial (Variables|Default|GetMast) 0 "/Game/Assets/Materials/M_ShipWood.M_ShipWood")
      (Variables|Default|SetCurrentWorkingStage "NewEnumerator6")
      (Utilities|Array|Clear _currentrequirements_2)
      (for _array_element_2 (Variables|STATICDATA|GetFlagReqs)
        (Utilities|Array|Add _currentrequirements_2 _array_element_2)))
    (:NewEnumerator6
      (Rendering|Material|SetMaterial (Variables|Default|GetFlag) 0 "/Game/Assets/Materials/M_ShipCloth.M_ShipCloth")
      (Variables|Default|SetCurrentWorkingStage "NewEnumerator6"))))

(fn UpdateUI
  (Default|RefreshRequirements (Variables|Default|GetRequirementsUI) (Variables|Default|GetCurrentRequirements)))

(fn ShipRepaired)

(fn CheckPlayerInventory
  (params (inReqs :type Array%20of%20S%20Ship%20Requirements%20Structures))
  (bind _as_player (Variables|Default|GetAs%20PLAYER))
  (bind _bpc_inventory (Variables|/Game/Player/_PLAYER._PLAYER_C|GetBPC_Inventory _as_player))
  (for (_array_element _array_index) inReqs
    (bind _returnvalue (Utilities|GetDataTableRow (.DataTable (Utilities|Struct|BreakDataTableRowHandle (.Items (Utilities|Struct|BreaksShipRequirements _array_element)))) (.RowName (Utilities|Struct|BreakDataTableRowHandle (.Items (Utilities|Struct|BreaksShipRequirements _array_element)))))
      (:then
        (for _index (range 1 (- (.AmountRequired (Utilities|Struct|BreaksShipRequirements _array_element)) (.AmountLoaded (Utilities|Struct|BreaksShipRequirements _array_element)))) ; cycles for as many are required at that point
          (bind (_found _founditem) (Default|CheckforItem _bpc_inventory (.ItemName (Utilities|Struct|BreaksItem _returnvalue))))
          (if _found
            (Default|RemoveItem _bpc_inventory _founditem)
            (Math|Integer|IncrementInt (LocalVariables|GetItemsRemoved))))
        (Utilities|Array|SetArrayElem inReqs _array_index (Utilities|Struct|MakesShipRequirements (.Items (Utilities|Struct|BreaksShipRequirements _array_element)) (+ (LocalVariables|GetItemsRemoved) (.AmountLoaded (Utilities|Struct|BreaksShipRequirements _array_element))) (.AmountRequired (Utilities|Struct|BreaksShipRequirements _array_element))))
        (LocalVariables|SetItemsRemoved 0)))))

(fn CheckifReqsMet
  (LocalVariables|SetMissingReq false)
  (for _array_element (Variables|Default|GetCurrentRequirements)
    (if (not (== (.AmountLoaded (Utilities|Struct|BreaksShipRequirements _array_element)) (.AmountRequired (Utilities|Struct|BreaksShipRequirements _array_element))))
      (LocalVariables|SetMissingReq true)))
  (if (not (LocalVariables|GetMissingReq))
    (CallFunction|NextStage (Variables|Default|GetCurrentWorkingStage))
    (CallFunction|UpdateUI)))