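; Trigger zone that switches the player's camera and the background music when the player overlaps its box.
; It passes the isometric flag, a third-person locator position and itself to the player's ChangeCamera, then has the MusicController loop the dusk theme for isometric zones or the restaurant theme otherwise.
; A separate ToggleVis event flips visibility and updates collision on a list of assigned actors.
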(event OnComponentBeginOverlap(Box)
  (params (OverlappedComponent :type Primitive%20Component%20Object%20Reference) (OtherActor :type Actor%20Object%20Reference) (OtherComp :type Primitive%20Component%20Object%20Reference) (OtherBodyIndex :type Integer) (bFromSweep :type Boolean) (SweepResult :type Hit%20Result%20Structure%20%28by%20ref%29))
  (bind _isiso (Variables|Default|GetisIso))
  (bind _as_player (Utilities|Casting|CastTo_PLAYER OtherActor))
  (Default|ChangeCamera _as_player _isiso (Transformation|GetWorldLocation (Variables|Default|GetTPLocator)) self false)
  (if _isiso
    (bind _returnvalue (Actor|GetActorOfClass "/Game/Tech/MusicController/MusicController.MusicController_C"))
    (Default|StopCurrentTrack _returnvalue)
    (Default|PlayTrackwithCue _returnvalue "/Game/Assets/Audio/Sounds/Music/Cues/Dusk_Theme_Cue.Dusk_Theme_Cue" true)
    (else
      (bind _returnvalue_2 (Actor|GetActorOfClass "/Game/Tech/MusicController/MusicController.MusicController_C"))
      (Default|StopCurrentTrack _returnvalue_2)
      (Default|PlayTrackwithCue _returnvalue_2 "/Game/Assets/Audio/Sounds/Music/Cues/Restaurant_Base_Cue.Restaurant_Base_Cue" true))))

(event Custom|ToggleVis
  (for _array_element (Variables|Default|GetAssetsToToggleVisibility)
    (Utilities|IsValid _array_element
      (:Is%20Valid
        (Rendering|SetActorHiddenInGame _array_element (not (Variables|/Script/Engine.Actor|GetbHidden _array_element)))
        (Collision|SetActorEnableCollision _array_element (not (Variables|/Script/Engine.Actor|GetbHidden _array_element)))))))

(fn ConstructionScript)