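; Component that runs a cooking stir QTE, where the player holds Left or Right to match a randomly chosen stir direction.
; StartCooking shows WB_CycleQTE and enables Tick, which feeds the required key state into StirringLoop.
; Holding correctly past a random interval flips the direction until the flip total is reached, while not holding builds BoilTimer toward failure.
; Success and failure only print a message, then End disables Tick and removes the widget.
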(event Custom|StartCooking
  (params (TotalFlips :type Byte) (OverCookedTime :type Float%20%28double-precision%29) (FlipTimeMax :type Float%20%28double-precision%29) (FlipTimeMin :type Float%20%28double-precision%29))
  (bind _widget (Variables|Default|Getwidget))
  ;[1 0.02353 0] Start
  (Variables|Default|SetFlipTotal TotalFlips)
  (Variables|Default|SetFailTime OverCookedTime)
  (Variables|Default|SetSwitchTimerMax FlipTimeMax)
  (Variables|Default|SetSwitchTimerMin FlipTimeMin)
  (Variables|Default|SetClockwise (Math|Random|RandomBool))
  (Variables|Default|SetFlipAt (Math|Random|RandomFloatinRange (Variables|Default|GetSwitchTimerMin) (Variables|Default|GetSwitchTimerMax)))
  (Components|Tick|SetComponentTickEnabled true)
  (Default|FlipImage _widget (Variables|Default|GetClockwise))
  (UserInterface|Viewport|AddtoViewport _widget 0))

(event Custom|End
  ;[1 0 0.01829] End
  (Components|Tick|SetComponentTickEnabled false)
  (Variables|Default|SetFlipAt 0.0)
  (Variables|Default|SetFlipCount 0)
  (Widget|RemovefromParent (Variables|Default|Getwidget)))

(event Custom|Flip
  ;[1 0 0.8683] Flip
  (bind _output_get (Variables|Default|SetFlipCount (+ (Variables|Default|GetFlipCount) 1)))
  (if (>= _output_get (Variables|Default|GetFlipTotal))
    (Development|PrintString "success")
    (CallFunction|End)
    (else
      (bind _output_get_2 (Variables|Default|SetClockwise (not (Variables|Default|GetClockwise))))
      (Default|FlipImage (Variables|Default|Getwidget) _output_get_2)
      (Variables|Default|SetTimer 0.0)
      (Variables|Default|SetFlipAt (Math|Random|RandomFloatinRange (Variables|Default|GetSwitchTimerMin) (Variables|Default|GetSwitchTimerMax))))))

(event EventBeginPlay
  (bind _returnvalue (UserInterface|CreateWidget "/Game/Blueprints/QTE/WB_CycleQTE.WB_CycleQTE_C" (Game|GetPlayerController 0)))
  (Variables|Default|Setwidget _returnvalue))

(event EventTick
  (params (DeltaSeconds :type Float%20%28single-precision%29))
  ;[0 0.884 1] Update
  (Variables|Default|SetTimer (+ DeltaSeconds (Variables|Default|GetTimer)))
  (if (Variables|Default|GetClockwise)
    (CallFunction|StirringLoop (Variables|Default|GetRightHeld))
    (Development|PrintString "right")
    (else
      (CallFunction|StirringLoop (Variables|Default|GetLeftHeld))
      (Development|PrintString "Left"))))

(event Input|KeyboardEvents|Left
  (params (Key :type Key%20Structure :default "None"))
  ;[1 0.8254 0] Input
  (:Pressed
    (Variables|Default|SetLeftHeld true))
  (:Released
    (Variables|Default|SetLeftHeld false)))

(event Input|KeyboardEvents|Right
  (params (Key :type Key%20Structure :default "None"))
  ;[1 0.8254 0] Input
  (:Pressed
    (Variables|Default|SetRightHeld true))
  (:Released
    (Variables|Default|SetRightHeld false)))

(fn StirringLoop
  (params (Held :type Boolean))
  (if Held
    ;[0 1 0.9709] Check for flip
    (if (<= (Variables|Default|GetBoilTimer) 0.0)
      (Variables|Default|SetBoilTimer 0.0)
      (else
        (Variables|Default|SetBoilTimer (- (Utilities|Time|GetWorldDeltaSeconds) (Variables|Default|GetBoilTimer)))))
    (if (>= (Variables|Default|GetTimer) (Variables|Default|GetFlipAt))
      (CallFunction|Flip))
    (else
      ;[1 0.02435 0] Check if fail
      (Variables|Default|SetBoilTimer (+ (Variables|Default|GetBoilTimer) (Utilities|Time|GetWorldDeltaSeconds)))
      (if (>= (Variables|Default|GetBoilTimer) (Variables|Default|GetFailTime))
        (Development|PrintString "Fail")
        (CallFunction|End)))))