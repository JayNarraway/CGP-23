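; BP_PotQTE is a work-in-progress cooking pot quick-time event where the player holds Left or Right to match the Clockwise flag.
; StartCooking enables Tick, which adjusts BoilTimer while the matching key is held, otherwise raises it until failure.
; CustomEvent flips direction or reports success, but nothing here calls it or increments FlipCount.
; Both keys set LeftHeld, the held-key subtraction is reversed, and the switch-timer check leads nowhere.
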(event Custom|StartCooking
  (Actor|Tick|SetActorTickEnabled true))

(event Custom|CustomEvent
  (if (>= (Variables|Default|GetFlipCount) (Variables|Default|GetFlipTotal))
    (Development|PrintString "Success")
    (Actor|Tick|SetActorTickEnabled false)
    (else
      (Variables|Default|SetClockwise (not (Variables|Default|GetClockwise)))
      (Variables|Default|SetTimer 0.0))))

(event EventBeginPlay)

(event Collision|EventActorBeginOverlap
  (params (OtherActor :type Actor%20Object%20Reference)))

(event EventTick
  (params (DeltaSeconds :type Float%20%28single-precision%29))
  (bind _returnvalue (Utilities|Time|GetWorldDeltaSeconds))
  (Variables|Default|SetTimer (+ DeltaSeconds (Variables|Default|GetTimer)))
  (if (Variables|Default|GetClockwise)
    (if (Variables|Default|GetRightHeld)
      (if (<= (stale _output_get) 0.0) :!label _label
        (Variables|Default|SetBoilTimer 0.0)
        (else
          (Variables|Default|SetBoilTimer (- _returnvalue (stale _output_get)))))
      (if (>= (Variables|Default|GetTimer) (Variables|Default|GetSwitchTimerMin))
        _)
      (else
        (bind _output_get (Variables|Default|SetBoilTimer (+ (Variables|Default|GetBoilTimer) _returnvalue) :!label _label_2))
        (if (>= (Variables|Default|GetBoilTimer) (Variables|Default|GetFailTime))
          (Development|PrintString "Fail")
          (Actor|Tick|SetActorTickEnabled false))))
    (elif (Variables|Default|GetLeftHeld)
      (goto _label)
      (else
        (goto _label_2)))))

(event Input|KeyboardEvents|Left
  (params (Key :type Key%20Structure :default "None"))
  (:Pressed
    (Variables|Default|SetLeftHeld true))
  (:Released
    (Variables|Default|SetLeftHeld false)))

(event Input|KeyboardEvents|Right
  (params (Key :type Key%20Structure :default "None"))
  (:Pressed
    (Variables|Default|SetLeftHeld true))
  (:Released
    (Variables|Default|SetLeftHeld false)))

(fn ConstructionScript)