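; Quick-time event logic component that times a single player press against a target window and signals success or fail.
; StartQTE creates the HUD widget, opens an input gate and starts a duration timer plus a looping timer that moves the icon.
; IA_QTE ends the QTE and checks elapsed time against the window; timeout just ends it, without signalling fail.
; Start's random-window calculation feeds only disconnected legacy logic.
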(event Custom|Start
  (bind _rangemin (Variables|OLD|GetRangeMin))
  (bind _rangemax (Variables|OLD|GetRangeMax))
  (bind _deltarange (Variables|OLD|GetDeltaRange))
  ;[0.5208 0.09437 0] Finds Acceptable Interact value
  (Variables|OLD|SetCurrTime 0.0)
  (Variables|OLD|SetCenterVal (Math|Random|RandomFloatinRange _rangemin _rangemax))
  (if (< (- (Variables|OLD|GetCenterVal) _deltarange) _rangemin)
    (bind _output_get (Variables|OLD|SetInteractMin (Variables|OLD|GetRangeMin)))
    (Variables|OLD|SetInteractMax (+ (* (Variables|OLD|GetDeltaRange) 2.0) _output_get))
    (elif (> (+ (Variables|OLD|GetCenterVal) _deltarange) _rangemax)
      (bind _output_get_2 (Variables|OLD|SetInteractMax (Variables|OLD|GetRangeMax)))
      (Variables|OLD|SetInteractMin (- _output_get_2 (* (Variables|OLD|GetDeltaRange) 2.0)))
      (else
        (Variables|OLD|SetInteractMax (+ (Variables|OLD|GetCenterVal) _deltarange))
        (Variables|OLD|SetInteractMin (- (Variables|OLD|GetCenterVal) _deltarange))))))

(event Custom|StartQTE
  (params (DistanceFromEnd :type Float%20%28double-precision%29) (MaxDuration :type Float%20%28double-precision%29) (Range :type Float%20%28double-precision%29))
  (bind _returnvalue (- MaxDuration DistanceFromEnd))
  (bind _returnvalue_2 (Utilities|Time|SetTimerbyEvent (delegate Custom|EndQTE) MaxDuration)) ; waits for however long Max Duration is
  (bind _ui_qte (Default|CreateQTE (Variables|/Game/Player/_PLAYER._PLAYER_C|GetAsHUD (stale EventBeginPlay _as_player)) DistanceFromEnd MaxDuration Range))
  (Utilities|IsValid (Variables|Default|GetUI%20QTE)
    (:Is%20Valid
      _)
    (:Is%20Not%20Valid
      (Variables|Default|SetUI%20QTE _ui_qte)))
  (bind _returnvalue_3 (Utilities|Time|SetTimerbyEvent (delegate Custom|UI%20Main%20Update) (Variables|Default|GetUIUpdateRate) true)) ; exists only to update UI
  (Utilities|FlowControl|Gate true) ; enters at Open
)

(event Custom|EndQTE
  (Utilities|Time|ClearandInvalidateTimerbyHandle (stale Custom|StartQTE _returnvalue_3)) ; stopst the UI Main Update
  (Utilities|FlowControl|Gate true) ; enters at Close
)

(event Custom|UI%20Main%20Update
  (Default|MoveIcon (Variables|Default|GetUI%20QTE) (Class|KismetSystemLibrary|GetTimerElapsedTimeHandle (stale Custom|StartQTE _returnvalue_2)) (stale Custom|StartQTE MaxDuration)))

(event Input|EnhancedActionEvents|EnhancedInputActionIA_QTE
  (params (ActionValue :type Boolean) (ElapsedSeconds :type Float%20%28double-precision%29) (TriggeredSeconds :type Float%20%28double-precision%29) (InputAction :type Input%20Action%20Object%20Reference :default "/Game/Input/Actions/IA_QTE.IA_QTE"))
  (:Started
    (Utilities|FlowControl|Gate true ; only allows input if QTE is active
      (:Exit
        ;[1 1 1] whatever logic you want to happen after the QTE comes after the "EndQTE" call
        (CallFunction|EndQTE)
        (if (Math|Float|InRange(Float) (Class|KismetSystemLibrary|GetTimerElapsedTimeHandle (stale Custom|StartQTE _returnvalue_2)) (- (- (stale Custom|StartQTE MaxDuration) (stale Custom|StartQTE DistanceFromEnd)) (stale Custom|StartQTE Range)) (+ (- (stale Custom|StartQTE MaxDuration) (stale Custom|StartQTE DistanceFromEnd)) (stale Custom|StartQTE Range)))
          (Default|CallQTESuccess)
          (else
            (Default|CallQTEFail)))))))

(event EventBeginPlay
  (bind _as_player (Utilities|Casting|CastTo_PLAYER (Game|GetPlayerCharacter 0)))
  (Variables|Default|SetAs%20HUD (Variables|/Game/Player/_PLAYER._PLAYER_C|GetAsHUD _as_player)))

(event EventTick
  (params (DeltaSeconds :type Float%20%28single-precision%29))
  ;[1 1 1] Update
)

(event Input|KeyboardEvents|E
  (params (Key :type Key%20Structure :default "None")))