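; BP_QTEBase is a quick time event Blueprint that tests whether E is pressed inside a randomly placed timing window.
; Start resets the timer and picks a window center, shifting the window to keep its width within the range limits.
; While Running, Tick advances the timer until it reaches Speed, a duration despite its name.
; Pressing E compares normalized time to the window, prints the result and clears Running.
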(event Custom|Start
  (bind _rangemin (Variables|Default|GetRangeMin))
  (bind _rangemax (Variables|Default|GetRangeMax))
  (bind _acceptablerange (Variables|Default|GetAcceptableRange))
  ;[0.5208 0.09437 0] Finds Acceptable Interact value
  (Variables|Default|SetCurrTime 0.0)
  (Variables|Default|SetCenterVal (Math|Random|RandomFloatinRange _rangemin _rangemax))
  (if (< (- (Variables|Default|GetCenterVal) _acceptablerange) _rangemin)
    (bind _output_get (Variables|Default|SetInteractMin (Variables|Default|GetRangeMin)))
    (Variables|Default|SetInteractMax (+ (* (Variables|Default|GetAcceptableRange) 2.0) _output_get))
    (elif (> (+ (Variables|Default|GetCenterVal) _acceptablerange) _rangemax)
      (bind _output_get_2 (Variables|Default|SetInteractMax (Variables|Default|GetRangeMax)))
      (Variables|Default|SetInteractMin (- _output_get_2 (* (Variables|Default|GetAcceptableRange) 2.0)))
      (else
        (Variables|Default|SetInteractMax (+ (Variables|Default|GetCenterVal) _acceptablerange))
        (Variables|Default|SetInteractMin (- (Variables|Default|GetCenterVal) _acceptablerange))))))

(event EventTick
  (params (DeltaSeconds :type Float%20%28single-precision%29))
  ;[1 1 1] Update
  (if (Variables|Default|GetRunning)
    (if (>= (Variables|Default|GetCurrTime) (Variables|Default|GetSpeed))
      (Development|PrintString "Too slow")
      (Variables|Default|SetRunning false)
      (else
        (Variables|Default|SetCurrTime (+ DeltaSeconds (Variables|Default|GetCurrTime)))))))

(event Input|KeyboardEvents|E
  (params (Key :type Key%20Structure :default "None"))
  (bind _currtime (Variables|Default|GetCurrTime))
  (bind _speed (Variables|Default|GetSpeed))
  (bind _returnvalue (/ _currtime _speed))
  (:Pressed
    (if (and (>= _returnvalue (Variables|Default|GetInteractMin)) (<= _returnvalue (Variables|Default|GetInteractMax)))
      (Development|PrintString "Success")
      (else
        (Development|PrintString "Fail")))
    (Variables|Default|SetRunning false)))

(fn ConstructionScript)