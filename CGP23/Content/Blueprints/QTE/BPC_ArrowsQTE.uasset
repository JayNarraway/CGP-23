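; Component that runs a timed arrow-key QTE for cooking, turning an inventory item into its recipe output or burned food.
; StartCook removes an item with linked chop data, switches input to IMC_QTE and shows a random arrow sequence in WB_ArrowQTE.
; Tick times each arrow; inputs or timeouts color it and advance.
; EndCooking adds the DataTable result based on mistake count, then restores perspective through the controller.
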(event Custom|StartCook
  (params (total%20arrows :type Integer) (time%20per%20input :type Float%20%28double-precision%29) (InItem :type S%20Item%20Structure))
  (bind _returnvalue (Game|GetPlayerController 0))
  (bind _widget (Variables|Default|GetWidget))
  (bind _returnvalue_2 (PlayerController|LocalPlayerSubsystems|GetEnhancedInputLocalPlayerSubsystem _returnvalue))
  (bind _success (CallFunction|HandleItemin InItem))
  ;[1 0.3483 0] start
  (if _success
    (Variables|Default|SetRunning true)
    (Variables|Default|SetTimeLimit time%20per%20input)
    (bind _output_get (Variables|Default|SetSize total%20arrows))
    (for _index (range 1 _output_get)
      (Utilities|Array|Add (Variables|Default|GetElements) (Math|Conversions|ToByte(Integer) (Math|Random|RandomIntegerinRange 0 3))))
    (Input|RemoveMappingContext _returnvalue_2 "/Game/Input/IMC_2D.IMC_2D" "(bIgnoreAllPressedKeysUntilRelease=True,bForceImmediately=False)")
    (Input|RemoveMappingContext _returnvalue_2 "/Game/Input/IMC_ISO.IMC_ISO" "(bIgnoreAllPressedKeysUntilRelease=True,bForceImmediately=False)") ; ADDED
    (Input|AddMappingContext _returnvalue_2 "/Game/Input/IMC_QTE.IMC_QTE" 0 "(bIgnoreAllPressedKeysUntilRelease=True,bForceImmediately=False)")
    (Components|Tick|SetComponentTickEnabled true)
    (for _array_element (Variables|Default|GetElements)
      (Default|CreateArrows _widget (Math|Conversions|ToInteger(Byte) _array_element)))
    (UserInterface|Viewport|AddtoViewport _widget 0)
    (bind _aswb_base_arrow (Utilities|Casting|CastToWB_BaseArrow (Class|PanelWidget|GetChildat (Variables|/Game/Blueprints/QTE/WB_ArrowQTE.WB_ArrowQTE_C|GetArrowsGrid (Variables|Default|GetWidget)) (Variables|Default|GetTarget))))
    (Default|SetActive _aswb_base_arrow true)))

(event Custom|End%20Cooking
  (bind _widget (Variables|Default|GetWidget))
  ;[0.474 0 0] End
  (CallFunction|SpawnItem (<= (Variables|Default|GetNumIncorrect) (Variables|Default|GetMaxFuckUps)))
  (Variables|Default|SetNumIncorrect 0)
  (Default|ReturnPerspective (Variables|Default|GetAs%20CONTROLLER) true)
  (Components|Tick|SetComponentTickEnabled false)
  (Widget|RemovefromParent _widget)
  (Utilities|Array|Clear (Variables|Default|GetElements))
  (Variables|Default|SetTarget 0)
  (Default|DestoryChildren _widget)
  (Variables|Default|SetRunning false))

(event Custom|Punish
  ;[0.92 0 1] Punishment or success
  (Development|PrintString "wrong")
  (bind _aswb_base_arrow (Utilities|Casting|CastToWB_BaseArrow (Class|PanelWidget|GetChildat (Variables|/Game/Blueprints/QTE/WB_ArrowQTE.WB_ArrowQTE_C|GetArrowsGrid (Variables|Default|GetWidget)) (Variables|Default|GetTarget))))
  (Default|ChangeColour _aswb_base_arrow "(R=0.255208,G=0.009808,B=0.000000,A=1.000000)")
  (Default|SetActive _aswb_base_arrow false)
  (Math|Integer|IncrementInt (Variables|Default|GetNumIncorrect)
    (:%20%20
      (CallFunction|IncrementElement))))

(event Custom|Correct
  ;[0.92 0 1] Punishment or success
  (Development|PrintString "correct")
  (bind _aswb_base_arrow (Utilities|Casting|CastToWB_BaseArrow (Class|PanelWidget|GetChildat (Variables|/Game/Blueprints/QTE/WB_ArrowQTE.WB_ArrowQTE_C|GetArrowsGrid (Variables|Default|GetWidget)) (Variables|Default|GetTarget))))
  (Default|ChangeColour _aswb_base_arrow "(R=0.000000,G=0.255208,B=0.009866,A=1.000000)")
  (Default|SetActive _aswb_base_arrow false)
  (CallFunction|IncrementElement))

(event Input|EnhancedActionEvents|EnhancedInputActionIA_Down
  (params (ActionValue :type Boolean) (ElapsedSeconds :type Float%20%28double-precision%29) (TriggeredSeconds :type Float%20%28double-precision%29) (InputAction :type Input%20Action%20Object%20Reference :default "/Game/Input/Actions/QTEActions/IA_Down.IA_Down"))
  ;[1 0.9868 0] inputs
  (:Started
    (Variables|Default|SetDown true)
    (if (Variables|Default|GetRunning)
      (switch int (Math|Conversions|ToInteger(Byte) (Utilities|Array|Get(acopy) (Variables|Default|GetElements) (Variables|Default|GetTarget)))
        (:0
          (CallFunction|InputCheck (Variables|Default|GetUp)))
        (:1
          (CallFunction|InputCheck (Variables|Default|GetRight)))
        (:2
          (CallFunction|InputCheck (Variables|Default|GetDown)))
        (:3
          (CallFunction|InputCheck (Variables|Default|GetLeft))))
      (Variables|Default|SetRight false)
      (Variables|Default|SetUp false)
      (Variables|Default|SetDown false)
      (Variables|Default|SetLeft false))))

(event Input|EnhancedActionEvents|EnhancedInputActionIA_Up
  (params (ActionValue :type Boolean) (ElapsedSeconds :type Float%20%28double-precision%29) (TriggeredSeconds :type Float%20%28double-precision%29) (InputAction :type Input%20Action%20Object%20Reference :default "/Game/Input/Actions/QTEActions/IA_Up.IA_Up"))
  ;[1 0.9868 0] inputs
  (:Started
    (Variables|Default|SetUp true)
    (if (Variables|Default|GetRunning)
      (switch int (Math|Conversions|ToInteger(Byte) (Utilities|Array|Get(acopy) (Variables|Default|GetElements) (Variables|Default|GetTarget)))
        (:0
          (CallFunction|InputCheck (Variables|Default|GetUp)))
        (:1
          (CallFunction|InputCheck (Variables|Default|GetRight)))
        (:2
          (CallFunction|InputCheck (Variables|Default|GetDown)))
        (:3
          (CallFunction|InputCheck (Variables|Default|GetLeft))))
      (Variables|Default|SetRight false)
      (Variables|Default|SetUp false)
      (Variables|Default|SetDown false)
      (Variables|Default|SetLeft false))))

(event Input|EnhancedActionEvents|EnhancedInputActionIA_Right
  (params (ActionValue :type Boolean) (ElapsedSeconds :type Float%20%28double-precision%29) (TriggeredSeconds :type Float%20%28double-precision%29) (InputAction :type Input%20Action%20Object%20Reference :default "/Game/Input/Actions/QTEActions/IA_Right.IA_Right"))
  ;[1 0.9868 0] inputs
  (:Started
    (Variables|Default|SetRight true)
    (if (Variables|Default|GetRunning)
      (switch int (Math|Conversions|ToInteger(Byte) (Utilities|Array|Get(acopy) (Variables|Default|GetElements) (Variables|Default|GetTarget)))
        (:0
          (CallFunction|InputCheck (Variables|Default|GetUp)))
        (:1
          (CallFunction|InputCheck (Variables|Default|GetRight)))
        (:2
          (CallFunction|InputCheck (Variables|Default|GetDown)))
        (:3
          (CallFunction|InputCheck (Variables|Default|GetLeft))))
      (Variables|Default|SetRight false)
      (Variables|Default|SetUp false)
      (Variables|Default|SetDown false)
      (Variables|Default|SetLeft false))))

(event Input|EnhancedActionEvents|EnhancedInputActionIA_Left
  (params (ActionValue :type Boolean) (ElapsedSeconds :type Float%20%28double-precision%29) (TriggeredSeconds :type Float%20%28double-precision%29) (InputAction :type Input%20Action%20Object%20Reference :default "/Game/Input/Actions/QTEActions/IA_Left.IA_Left"))
  ;[1 0.9868 0] inputs
  (:Started
    (Variables|Default|SetLeft true)
    (if (Variables|Default|GetRunning)
      (switch int (Math|Conversions|ToInteger(Byte) (Utilities|Array|Get(acopy) (Variables|Default|GetElements) (Variables|Default|GetTarget)))
        (:0
          (CallFunction|InputCheck (Variables|Default|GetUp)))
        (:1
          (CallFunction|InputCheck (Variables|Default|GetRight)))
        (:2
          (CallFunction|InputCheck (Variables|Default|GetDown)))
        (:3
          (CallFunction|InputCheck (Variables|Default|GetLeft))))
      (Variables|Default|SetRight false)
      (Variables|Default|SetUp false)
      (Variables|Default|SetDown false)
      (Variables|Default|SetLeft false))))

(event EventTick
  (params (DeltaSeconds :type Float%20%28single-precision%29))
  ;[0 0.9893 1] Update
  (if (>= (Variables|Default|GetTimer) (Variables|Default|GetTimeLimit))
    (CallFunction|Punish)
    (else
      (Variables|Default|SetTimer (+ DeltaSeconds (Variables|Default|GetTimer))))))

(event EventBeginPlay
  ;[0.3052 1 0] Begin Play
  (bind _returnvalue (UserInterface|CreateWidget "/Game/Blueprints/QTE/WB_ArrowQTE.WB_ArrowQTE_C" (Game|GetPlayerController 0)))
  (Variables|Default|SetWidget _returnvalue)
  (bind _as_controller (Utilities|Casting|CastTo_CONTROLLER (Game|GetPlayerController 0)))
  (Variables|Default|SetAs%20CONTROLLER _as_controller))

(fn InputCheck
  (params (Input :type Boolean))
  (if Input
    (CallFunction|Correct)
    (else
      (CallFunction|Punish))))

(fn IncrementElement
  (bind _result (Math|Integer|IncrementInt (Variables|Default|GetTarget))
    (:%20%20
      (Variables|Default|SetTimer 0.0)
      (if (>= _result (Variables|Default|GetSize))
        (CallFunction|EndCooking)
        (else
          (Development|PrintString (Utilities|String|ToString(Byte) (Utilities|Array|Get(acopy) (Variables|Default|GetElements) (Variables|Default|GetTarget))))
          (bind _aswb_base_arrow (Utilities|Casting|CastToWB_BaseArrow (Class|PanelWidget|GetChildat (Variables|/Game/Blueprints/QTE/WB_ArrowQTE.WB_ArrowQTE_C|GetArrowsGrid (Variables|Default|GetWidget)) (Variables|Default|GetTarget))))
          (Default|SetActive _aswb_base_arrow true))))))

(fn HandleItemin
  (params (InItem :type S%20Item%20Structure))
  (bind (_itemname _texture _amount_shouldbe1 _isstackable _maxstack _mesh _linkedgrowdata _linkedovendata _linkedpotdata _linkedchopdata) (Utilities|Struct|BreaksItem InItem))
  (if (Utilities|Enum|Equal(Enum) _itemname (Utilities|Text|MakeLiteralText "AIR")) ; isnt an empty hand
    _
    (elif (not (== (.RowName (Utilities|Struct|BreakDataTableRowHandle _linkedchopdata)) "EMPTY")) ; has a linked chop
      (bind _output_get (Variables|Default|SetIn%20Item InItem))
      (bind _itemremoved (Default|RemoveItem (.OwningInventory-IGNORE (Utilities|Struct|BreaksItem _output_get)) _output_get))
      (if _itemremoved
        (return true)
        (else
          (return false)))
      (else
        _)))
  (return false))

(fn SpawnItem
  (params (isSuccess :type Boolean))
  (bind _in_item (Variables|Default|GetIn%20Item))
  (bind (_itemname _texture _amount_shouldbe1 _isstackable _maxstack _mesh _linkedgrowdata _linkedovendata _linkedpotdata _linkedchopdata _itemquality_ignore _owninginventory_ignore) (Utilities|Struct|BreaksItem _in_item))
  (bind (_datatable _rowname) (Utilities|Struct|BreakDataTableRowHandle _linkedchopdata))
  (bind _returnvalue (Utilities|GetDataTableRow _datatable _rowname)
    (:then
      (bind _returnvalue_2 (Utilities|GetDataTableRow (.DataTable (Utilities|Struct|BreakDataTableRowHandle (select isSuccess (.OutputItem (Utilities|Struct|BreaksFood _returnvalue)) (Utilities|Struct|MakeDataTableRowHandle "/Game/Static_Data/Item/DT_Items.DT_Items" "BurnedFood")))) (.RowName (Utilities|Struct|BreakDataTableRowHandle (select isSuccess (.OutputItem (Utilities|Struct|BreaksFood _returnvalue)) (Utilities|Struct|MakeDataTableRowHandle "/Game/Static_Data/Item/DT_Items.DT_Items" "BurnedFood")))))
        (:then
          (Default|AddItemtoInventory _owninginventory_ignore _returnvalue_2))))))