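; Fishing lure actor that launches itself along the player's forward arrow on spawn, then raises linear damping after a short delay to slow down.
; On hit, the physics sphere activates a ripple effect while a timeline nudges it upward each update, deactivating the ripple when finished.
; A dynamic material starts bright red, turns green on FishReady and changes to the default MakeColor value on FishGone.
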(event OnComponentHit(Sphere)
  (params (HitComponent :type Primitive%20Component%20Object%20Reference) (OtherActor :type Actor%20Object%20Reference) (OtherComp :type Primitive%20Component%20Object%20Reference) (NormalImpulse :type Vector :default "0, 0, 0") (Hit :type Hit%20Result%20Structure%20%28by%20ref%29))
  (bind _sphere (Variables|Default|GetSphere))
  (bind _returnvalue (Transformation|GetWorldLocation _sphere))
  (Components|Activation|Activate (Variables|Default|GetNS_Ripple) false)
  (Timeline|Timeline PlayFromStart
    (:Update
      (Transformation|SetRelativeLocation _sphere (Math|Vector|Lerp(Vector) _returnvalue (+ _returnvalue "0.000000,0.000000,2.000000") 1.0) false false))
    (:Finished
      (Components|Activation|Deactivate (Variables|Default|GetNS_Ripple)))))

(event EventBeginPlay
  (bind _sphere (Variables|Default|GetSphere))
  (bind _returnvalue (Actor|GetActorOfClass "/Game/Player/_PLAYER._PLAYER_C"))
  (Class|PrimitiveComponent|AddVelocityChangeImpulseatLocation _sphere (* (Math|Vector|GetForwardVector (Variables|/Game/Player/_PLAYER._PLAYER_C|GetMesh%20Forward%20Vector _returnvalue)) "300.000000,300.000000,300.000000") (Variables|/Script/Engine.SceneComponent|GetRelativeLocation (Variables|/Script/Engine.Character|GetCapsuleComponent _returnvalue)) "None")
  (Utilities|FlowControl|Delay 0.5)
  (Class|PrimitiveComponent|SetLinearDamping _sphere 5.0))

(event EventFishReady
  (Rendering|Material|SetVectorParameterValue (Variables|Default|GetMaterialColour) "Colour" (Math|Color|MakeColor 0.0 1e+04 0.0) :!class /Script/Engine.MaterialInstanceDynamic))

(event EventFishGone
  (Rendering|Material|SetVectorParameterValue (Variables|Default|GetMaterialColour) "Colour" (Math|Color|MakeColor 0.0 0.0 0.0) :!class /Script/Engine.MaterialInstanceDynamic))

(fn ConstructionScript
  (bind _returnvalue (Rendering|Material|CreateDynamicMaterialInstance (Variables|Default|GetSphere) 0 "/Game/Blueprints/Interactables/Fishing_Visuals/M_DynamicColour.M_DynamicColour" "None" :!class /Script/Engine.PrimitiveComponent))
  (bind _output_get (Variables|Default|SetMaterialColour _returnvalue))
  (Rendering|Material|SetVectorParameterValue _output_get "Colour" (Math|Color|MakeColor 1e+04 0.0 0.0) :!class /Script/Engine.MaterialInstanceDynamic))