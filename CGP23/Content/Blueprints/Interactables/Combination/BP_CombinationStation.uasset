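; Interactable crafting station that opens the WBP_Combination widget, pausing the game and switching to UI-only input.
; RecieveOutput takes a recipe, calls BriamCheck on the tutorial door, then resolves two or three ingredients from data table row references.
; It checks the player's inventory for each, gathering matches in ItemsToRemove.
; If all are found, it removes them and spawns the output as a BP_BaseItem at the player's transform.
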(event Custom|RecieveOutput
  (params (Recipe :type S%20Combi%20Recipe%20Structure))
  (bind (_name _ingredientcount _stringredient1 _stringredient2 _stringredient3 _refoutput _refingredient1 _refingredient2 _refingredient3) (Utilities|Struct|BreaksCombiRecipe Recipe))
  (bind _itemstoremove (Variables|Default|GetItemsToRemove))
  (bind _itemstoremove_2 (Variables|Default|GetItemsToRemove))
  (bind _returnvalue (Actor|GetActorOfClass "/Game/Tutorial/A_TutorialDoor_Briam.A_TutorialDoor_Briam_C"))
  (Default|BriamCheck _returnvalue)
  (bind _item (CallFunction|GetItemfromRef _refingredient1))
  (bind (_success_ _itemtoremove) (CallFunction|TryRemoveItem _item))
  (if _success_
    (Utilities|Array|Add _itemstoremove _itemtoremove)
    (bind _item_2 (CallFunction|GetItemfromRef _refingredient2))
    (bind (_success__2 _itemtoremove_2) (CallFunction|TryRemoveItem _item_2))
    (if _success__2
      (Utilities|Array|Add _itemstoremove _itemtoremove_2)
      (if (> _ingredientcount 2)
        (bind _item_3 (CallFunction|GetItemfromRef _refingredient3))
        (bind (_success__3 _itemtoremove_3) (CallFunction|TryRemoveItem _item_3))
        (if _success__3
          (Utilities|Array|Add _itemstoremove_2 _itemtoremove_3)
          (for _array_element _itemstoremove_2 :!label _label
            (Default|RemoveItem (Variables|/Game/Player/_PLAYER._PLAYER_C|GetBPC_Inventory (Variables|Default|GetAs%20PLAYER)) _array_element))
          (Game|SpawnActorfromClass "/Game/Blueprints/Inventory/BP_BaseItem.BP_BaseItem_C" (Transformation|GetActorTransform (Variables|Default|GetAs%20PLAYER)) "Undefined" "MultiplyWithRoot" 0 _refoutput 0)
          (else
            (Development|PrintString "3rd not found")))
        (else
          (goto _label)))
      (else
        (Development|PrintString "2 not found")))
    (else
      (Development|PrintString "Not Found"))))

(event EventBeginPlay)

(event Collision|EventActorBeginOverlap
  (params (OtherActor :type Actor%20Object%20Reference)))

(event EventTick
  (params (DeltaSeconds :type Float%20%28single-precision%29)))

(event EventInteract
  (params (HitComponent :type Primitive%20Component%20Object%20Reference) (ItemInHand :type S%20Item%20Structure))
  (bind _returnvalue (UserInterface|CreateWidget "/Game/Blueprints/Interactables/Combination/WBP_Combination.WBP_Combination_C"))
  (UserInterface|Viewport|AddtoViewport _returnvalue 0)
  (Game|SetGamePaused true)
  (Input|SetInputModeUIOnly (Game|GetPlayerController 0) _returnvalue "DoNotLock" false))

(fn ConstructionScript
  (|CallParentFunction))

(fn GetItemfromRef
  (params (Ref :type Data%20Table%20Row%20Handle%20Structure))
  (bind (_datatable _rowname) (Utilities|Struct|BreakDataTableRowHandle Ref))
  (bind _returnvalue (Utilities|GetDataTableRow _datatable _rowname)
    (:then
      (return _returnvalue))))

(fn TryRemoveItem
  (params (Item%20In :type S%20Item%20Structure))
  (bind (_found _founditem) (Default|CheckforItem (Variables|/Game/Player/_PLAYER._PLAYER_C|GetBPC_Inventory (Variables|Default|GetAs%20PLAYER)) (.ItemName (Utilities|Struct|BreaksItem Item%20In))))
  (return _found _founditem))