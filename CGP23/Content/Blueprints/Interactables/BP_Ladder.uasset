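; Interactable ladder end that, paired with another ladder actor, automatically carries the player up or down between the two.
; On interact, it snaps the player to the ladder's X, locks the other end, disables character movement and sets a climb animation.
; A Timeline lerps the player along the up vector, negated unless GoingUp, by the distance to the other end.
; A DoOnce guards the climb until the Timeline finishes and restores movement and usability.
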(event Custom|ResetDoOnce
  (Variables|BP_Ladder_C|SetIsUsable (Variables|Default|GetLadder_Other) true)
  (Components|Activation|SetActive (Variables|/Script/Engine.Character|GetCharacterMovement (Variables|Default|GetAs%20PLAYER)) true false)
  (Utilities|FlowControl|DoOnce false) ; enters at Reset
)

(event EventInteract
  (params (HitComponent :type Primitive%20Component%20Object%20Reference) (ItemInHand :type S%20Item%20Struct%20Structure))
  (if (Variables|Default|GetIsUsable)
    (Transformation|SetActorLocation (Variables|Default|GetAs%20PLAYER) (Math|Vector|MakeVector (.x (Transformation|GetActorLocation (Variables|Default|GetLadder_Self))) (.y (Transformation|GetActorLocation (Variables|Default|GetAs%20PLAYER))) (.z (Transformation|GetActorLocation (Variables|Default|GetAs%20PLAYER)))) false false)
    (Variables|BP_Ladder_C|SetIsUsable (Variables|Default|GetLadder_Other) false)
    (Components|Activation|SetActive (Variables|/Script/Engine.Character|GetCharacterMovement (Variables|Default|GetAs%20PLAYER)) false false)
    (Components|Animation|SetAnimation (Variables|/Script/Engine.Character|GetMesh (Variables|Default|GetAs%20PLAYER)) "/Game/Animation/Anims/ladderclimb_Stationary.ladderclimb_Stationary")
    (Utilities|FlowControl|DoOnce false
      (:Completed
        (bind _output_get (Variables|Default|SetUpVector (Transformation|GetActorUpVector)))
        (if (Variables|Default|GetGoingUp)
          _
          (else
            (Variables|Default|SetUpVector (* _output_get "-1.000000,-1.000000,-1.000000"))))
        (bind _returnvalue (Actor|GetActorOfClass "/Game/Player/_PLAYER._PLAYER_C"))
        (bind _output_get_2 (Variables|Default|SetAs%20PLAYER _returnvalue))
        (Variables|Default|SetTargetPos (Transformation|GetActorLocation (Variables|Default|GetLadder_Other)))
        (Variables|Default|SetPlayerPos (Transformation|GetActorLocation _output_get_2))
        (Variables|Default|SetNextPos (+ (Variables|Default|GetPlayerPos) (* (Variables|Default|GetUpVector) (Transformation|GetDistanceTo self (Variables|Default|GetLadder_Other)))))
        (bind _uplerp (Timeline|Timeline PlayFromStart)
          (:Update
            (Transformation|SetActorLocation (Variables|Default|GetAs%20PLAYER) (Math|Vector|Lerp(Vector) (Variables|Default|GetPlayerPos) (Variables|Default|GetNextPos) _uplerp) false false))
          (:Finished
            (CallFunction|ResetDoOnce)))))))

(fn ConstructionScript
  (|CallParentFunction))