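; Master interactable Blueprint that starts a quick time event (QTE) when interacted with.
; Its interaction interface function calls StartQTE on the BPCQTELogic component with randomized distance from end, maximum duration and range.
; BeginPlay binds event delegates to that component's success and fail notifications.
; The QTE success and fail events only print debug strings.
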(event Custom|QTESuccess
  (Development|PrintString "QTE Success!"))

(event Custom|QTEFail
  (Development|PrintString "QTE Fail!"))

(event EventBeginPlay
  (bind _bpc_qtelogic (Variables|Default|GetBPC_QTELogic))
  (EventDispatchers|BindEventtoQTESuccess _bpc_qtelogic (EventDispatchers|CreateEvent :!event Custom|QTESuccess))
  (EventDispatchers|BindEventtoQTEFail _bpc_qtelogic (EventDispatchers|CreateEvent :!event Custom|QTEFail)))

(fn ConstructionScript
  (|CallParentFunction))

(fn InterfaceInteraction
  (params (interactingItem :type S%20Item%20Structure))
  (Default|StartQTE (Variables|Default|GetBPC_QTELogic) (Math|Random|RandomFloatinRange 0.5 1.0) (Math|Random|RandomFloatinRange 3.0 7.0) (Math|Random|RandomFloatinRange 0.1 0.2)))