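; Crop plot actor, still work-in-progress, that grows a crop through stages while watered and yields an item.
; Interact tries collecting, planting (hard-disabled), watering, then advancing growth; collecting resets the plot without granting items.
; GrowthMode scales one mesh or swaps stage meshes; HarvestMode spawns a BP_BaseItem or displays it for collection.
; Data table handles link items to growables; a literal/percentage mesh picker is only debug-printed on BeginPlay.
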(event Custom|ResetGrowthStage
  (Variables|Default|SetCurrentGrowthStage 0)
  (CallFunction|UpdateGrowableVisual)
  (Components|StaticMesh|SetStaticMesh (Variables|Default|GetPendingItem) 0))

(event Custom|SetGrowthStage
  (params (New%20Growth%20Stage :type Integer))
  (if (<= New%20Growth%20Stage (Variables|Default|GetGrowthStageLimit))
    (Variables|Default|SetCurrentGrowthStage New%20Growth%20Stage)
    (CallFunction|UpdateGrowableVisual)
    (else
      (Development|PrintString "Given number to set growth stage is larger than limit"))))

(event Custom|CompleteGrowthBasedOnHarvestMode
  (switch Utilities|FlowControl|Switch|SwitchonENM_HarvestModes (Variables|Default|GetHarvestMode)
    (:NewEnumerator0
      (CallFunction|SpawnGrowablesLinkedItem))
    (:NewEnumerator1
      (CallFunction|PresentGrowablesLinkedItem))))

(event Custom|SetWateredState
  (params (New%20Watered%20State :type Boolean))
  (Variables|Default|SetIsWatered New%20Watered%20State)
  (Development|PrintString "plant has been watered"))

(event Custom|SpawnGrowablesLinkedItem
  (params (Growable%20Input :type S%20Growable%20Structure))
  (bind _grownitem (Utilities|Struct|BreaksGrowable Growable%20Input))
  (bind (_datatable _rowname) (Utilities|Struct|BreakDataTableRowHandle _grownitem))
  ;[1 1 1] immediately ejects item, Used for walk into to pick up item
  (Class|DataTableFunctionLibrary|DoesDataTableRowExist _datatable _rowname)
  (if (!= _rowname "EMPTY")
    ;[1 1 1] need to spawn item but the object and class requires setting up for each instance spawning, need a premade thing to spawn without touching it
    (bind _returnvalue (Game|SpawnActorfromClass "/Game/Blueprints/Inventory/BP_BaseItem.BP_BaseItem_C" (Math|Transform|MakeTransform (.location (Transformation|GetWorldTransform (Variables|Default|GetArrow))) "0, 0, 0" (Class|KismetMathLibrary|VectorOne)) "Undefined" "MultiplyWithRoot" 0 (Utilities|Struct|MakeDataTableRowHandle _datatable _rowname) 0))
    (Components|StaticMesh|SetStaticMesh (Variables|/Game/Blueprints/Inventory/BP_BaseItem.BP_BaseItem_C|GetItemMesh _returnvalue) (.Mesh (Utilities|Struct|BreaksItem (CallFunction|GetItemfromGrowable Growable%20Input))))
    (Variables|Default|SetCanHarvest false)
    (CallFunction|ResetGrowthStage)))

(event Custom|PresentGrowablesLinkedItem
  (params (Growable%20Input :type S%20Growable%20Structure))
  (bind _grownitem (Utilities|Struct|BreaksGrowable Growable%20Input))
  (bind (_datatable _rowname) (Utilities|Struct|BreakDataTableRowHandle _grownitem))
  ;[1 1 1] presents item in a hold, Used for interact to harvest item
  (Variables|Default|SetCanHarvest true)
  (Class|DataTableFunctionLibrary|DoesDataTableRowExist _datatable _rowname)
  (if (!= _rowname "EMPTY")
    (Components|StaticMesh|SetStaticMesh (Variables|Default|GetPendingItem) (.Mesh (Utilities|Struct|BreaksItem (CallFunction|GetItemfromGrowable Growable%20Input))))))

(event Custom|CheckForCompletedGrowth
  (if (Math|Boolean|ANDBoolean (not (Variables|Default|GetCanHarvest)) (>= (Variables|Default|GetCurrentGrowthStage) (Variables|Default|GetGrowthStageLimit)) (Variables|Default|GetIsWatered))
    (CallFunction|CompleteGrowthBasedonHarvestMode)
    (else
      (Development|PrintString "conditions not jmet to complete growth"))))

(event Custom|IncrementGrowthStage
  (if (< (Variables|Default|GetCurrentGrowthStage) (Variables|Default|GetGrowthStageLimit))
    (if (Variables|Default|GetIsWatered)
      (bind _result (Math|Integer|IncrementInt (Variables|Default|GetCurrentGrowthStage))
        (:%20%20
          (Variables|Default|SetCurrentGrowthStage _result)
          (CallFunction|UpdateGrowableVisual)
          (CallFunction|CheckforCompletedGrowth)))
      (else
        (Development|PrintString "can't grow, not watered")))
    (elif true
      (Development|PrintString "Didin't increment growth stage, is already at limit")
      (else
        (CallFunction|CheckforCompletedGrowth)
        (CallFunction|UpdateGrowableVisual)))))

(event Custom|SetYieldMultiplier
  (params (New%20Multiplier :type Integer))
  (Variables|Default|SetYieldMultiplier New%20Multiplier))

(event Custom|CompileGrowthProperties
  (switch Utilities|FlowControl|Switch|SwitchonENM_GrowthModes (Variables|Default|GetGrowthMode)
    (:NewEnumerator0
      (if (Utilities|IsValid (Utilities|Array|Get(acopy) (Variables|Default|GetGrowthGraphics)))
        (Development|PrintString "Didin't reset mesh slot: Existing found")
        (else
          (Variables|Default|SetGrowthGraphics (Utilities|Array|MakeArray 0)))))
    (:NewEnumerator1
      (CallFunction|RecalculateMeshSlotsCount))))

(event Custom|SetGrowthStageLimit
  (params (New%20Growth%20Stage%20Limit :type Integer))
  (Variables|Default|SetGrowthStageLimit New%20Growth%20Stage%20Limit)
  (Development|PrintString (Utilities|String|ToString(Integer) (Variables|Default|GetGrowthStageLimit))))

(event Custom|SetCurrentGrowable
  (params (Growable%20Input :type S%20Growable%20Structure))
  (CallFunction|SetGrowthStageLimit (Math|Float|Truncate (.GrowTime (Utilities|Struct|BreaksGrowable Growable%20Input)))))

(event Custom|UpdateGrowableVisual
  ;[1 1 1] Call to update how the growing element looks. Do this after updating the data for the growing item's progression
  (switch Utilities|FlowControl|Switch|SwitchonENM_GrowthModes (Variables|Default|GetGrowthMode)
    (:NewEnumerator0
      (CallFunction|UpdateGrowableMeshScale))
    (:NewEnumerator1
      (CallFunction|UpdateGrowableMeshType))))

(event Custom|UpdateGrowableMeshScale
  (bind _currentgrowablemesh (Variables|Default|GetCurrentGrowableMesh))
  (if (Utilities|IsValid (Variables|/Script/Engine.StaticMeshComponent|GetStaticMesh (Variables|Default|GetCurrentGrowableMesh)))
    _
    (else
      (Variables|Default|SetGrowthGraphics (Utilities|Array|MakeArray 0))
      (Components|StaticMesh|SetStaticMesh _currentgrowablemesh 0)))
  (Transformation|SetRelativeScale3D _currentgrowablemesh (* (/ (Variables|Default|GetCurrentGrowthStage) (Variables|Default|GetGrowthStageLimit)) (Class|KismetMathLibrary|VectorOne))))

(event Custom|UpdateGrowableMeshType
  (Components|StaticMesh|SetStaticMesh (Variables|Default|GetCurrentGrowableMesh) (Utilities|Array|Get(acopy) (Variables|Default|GetGrowthGraphics) (Variables|Default|GetCurrentGrowthStage))))

(event EventBeginPlay
  (bind (_out_mesh _out_result) (CallFunction|GetCorrectMeshfromGrowable (Variables|Default|GetCurrentGrowthStage) (Variables|Default|GetGrowthStageLimit) (Variables|Default|GetGrowthGraphics)))
  (Development|PrintString (Utilities|String|Append "Got: " (Utilities|GetDisplayName _out_mesh) " with result " (Utilities|String|ToString(Boolean) _out_result))))

(event EventInteract
  (params (HitComponent :type Primitive%20Component%20Object%20Reference) (ItemInHand :type S%20Item%20Structure))
  (bind _growable_out (CallFunction|GetGrowablefromItem ItemInHand))
  (bind _out_result (CallFunction|CheckforCollection))
  ;[1 1 1] Condition for collecting
  (if _out_result
    (Development|PrintString "collecting")
    (bind _returnvalue (Actor|GetActorOfClass "/Game/Player/_PLAYER._PLAYER_C"))
    (bind _as_player (Utilities|Casting|CastTo_PLAYER _returnvalue)
      (:then
        (for _index (range 0 (Variables|Default|GetYieldMultiplier))
          _)
        (Development|PrintString (Utilities|String|ToString(Integer) _index))
        (Variables|Default|SetCanHarvest false)
        (CallFunction|ResetGrowthStage))
      (:CastFailed
        (Development|PrintString "cast to player on collect failed")))
    (else
      (bind _out_result_2 (CallFunction|CheckforPlanting ItemInHand))
      ;[1 1 1] Condition for planting
      (if _out_result_2
        (Development|PrintString (Class|BlueprintPathsLibrary|Combine (Utilities|Array|MakeArray "Planting: " (Utilities|String|ToString(Text) (.PlantName (Utilities|Struct|BreaksGrowable _growable_out))))))
        (CallFunction|SetCurrentGrowable _growable_out)
        (else
          (bind _out_result_3 (CallFunction|CheckforWatering ItemInHand))
          ;[1 1 1] Condition for watering
          (if _out_result_3
            (Development|PrintString "Hello")
            (CallFunction|SetWateredState true)
            (else
              (Development|PrintString "Crop can't detect a valid action to react")
              (CallFunction|IncrementGrowthStage))))))))

(fn ConstructionScript
  (Development|PrintString "Construction Script Ran")
  (CallFunction|CompileGrowthProperties)
  (|CallParentFunction))

(fn GetItemfromGrowable
  (params (Growable%20in :type S%20Growable%20Structure))
  (bind _grownitem (Utilities|Struct|BreaksGrowable Growable%20in))
  (bind (_datatable _rowname) (Utilities|Struct|BreakDataTableRowHandle _grownitem))
  (bind _returnvalue (Utilities|GetDataTableRow _datatable _rowname)
    (:then
      (if (!= _rowname "NULL")
        (return _returnvalue)
        (else
          (Development|PrintString "Failed to get item from growable"))))))

(fn GetGrowablefromItem
  (params (Item%20in :type S%20Item%20Structure))
  (bind _linkedgrowdata (Utilities|Struct|BreaksItem Item%20in))
  (bind (_datatable _rowname) (Utilities|Struct|BreakDataTableRowHandle _linkedgrowdata))
  (bind _returnvalue (Utilities|GetDataTableRow _datatable _rowname)
    (:then
      (if (!= _rowname "NULL")
        (return _returnvalue)
        (else
          (Development|PrintString "Failed to get growable from item"))))))

(fn CheckforCollection
  (return (Math|Boolean|ANDBoolean (Variables|Default|GetCanHarvest) (Utilities|Enum|Equal(Enum) (Variables|Default|GetHarvestMode) "NewEnumerator1") (not false))))

(fn CheckforPlanting
  (params (In%20Item :type S%20Item%20Structure))
  (return (and (Utilities|Enum|NotEqual(Enum) (.ItemName (Utilities|Struct|BreaksItem In%20Item)) (Utilities|Text|ToText(Name) (Variables|Default|GetEmptyItem))) false)))

(fn CheckforWatering
  (params (In%20Item :type S%20Item%20Structure))
  (bind _wateringitem (Variables|Default|GetWateringItem))
  (bind (_datatable _rowname) (Utilities|Struct|BreakDataTableRowHandle _wateringitem))
  (bind _returnvalue (Utilities|GetDataTableRow _datatable _rowname)
    (:then
      (return (Math|Boolean|ANDBoolean (Utilities|Enum|Equal(Enum) (Utilities|String|ToString(Text) (.ItemName (Utilities|Struct|BreaksItem _returnvalue))) (Utilities|String|ToString(Text) (.ItemName (Utilities|Struct|BreaksItem In%20Item)))) (not false) (not (Variables|Default|GetIsWatered)))))
    (:RowNotFound
      (Development|PrintString "Can't check for watering cause watering item name couldnt be found"))))

(fn RecalculateMeshSlotsCount
  (bind _array_element (Utilities|Array|ForEachLoopwithBreak (Variables|Default|GetGrowthGraphics))
    (:LoopBody
      (if (Utilities|IsValid _array_element)
        (LocalVariables|SetHasAnUnemptyGraphic true)))
    (:Completed
      (if (LocalVariables|GetHasAnUnemptyGraphic)
        (Development|PrintString "Graphic still assigned, not changing array length")
        (else
          (Variables|Default|SetGrowthGraphics (Utilities|Array|MakeArray))
          (for _index (range 0 (- (Variables|Default|GetGrowthStageLimit) (LocalVariables|GetArrayIndexOffset)))
            (Utilities|Array|AppendArray (Variables|Default|GetGrowthGraphics) (Utilities|Array|MakeArray 0))))))))

(fn GetCorrectMeshfromGrowable
  (params (In%20Current :type Integer) (In%20Limit :type Integer) (In%20Meshes%20%28Array%29 :type Array%20of%20Static%20Mesh%20Object%20References))
  (bind _output (Utilities|Array|Get(acopy) In%20Meshes%20%28Array%29))
  (bind _filteredarray (LocalVariables|GetFilteredArray))
  (bind _filteredarray_2 (LocalVariables|GetFilteredArray))
  (bind _returnvalue (Utilities|Array|Length _filteredarray_2))
  (bind _output_2 (Utilities|Array|Get(acopy) _filteredarray In%20Current))
  (switch Utilities|FlowControl|Switch|SwitchonENM_GrowthModes (Variables|Default|GetGrowthMode)
    (:NewEnumerator0
      ;[1 1 1] Get the only (first) mesh there is and if exists, return it
      (if (Utilities|IsValid _output)
        (return _output true)
        (else
          (return 0 false))))
    (:NewEnumerator1
      (switch Utilities|FlowControl|Switch|SwitchonENM_MeshAssignmentModes (Variables|Default|GetMeshAssignmentMode)
        (:NewEnumerator0
          ;[1 1 1] Get the mesh using the current growth stage as the index to look at and return if success
          (for _array_element In%20Meshes%20%28Array%29
            (if (Utilities|IsValid _array_element)
              (Utilities|Array|AppendArray (LocalVariables|GetFilteredArray) (Utilities|Array|MakeArray _array_element))))
          (if (Utilities|IsValid _output_2)
            (return _output_2 true)
            (else
              (return 0 false))))
        (:NewEnumerator1
          (for _array_element_2 In%20Meshes%20%28Array%29
            (if (Utilities|IsValid _array_element_2)
              (Utilities|Array|AppendArray (LocalVariables|GetFilteredArray) (Utilities|Array|MakeArray _array_element_2))))
          ;[1 1 1] Percent = (current / max) * 100
          (bind _output_get (LocalVariables|SetCurrentPercentage (* (/ In%20Current In%20Limit) 1e+02)))
          (Development|PrintString (Utilities|String|ToString(Float) _output_get) true true "(R=0.000000,G=0.660000,B=1.000000,A=1.000000)" 2e+01)
          ;[1 1 1] Runs on index first, last, and all inbetween
          (for _index (range 0 (- _returnvalue 1))
            (if (and (< (* _index (/ 100 _returnvalue)) (LocalVariables|GetCurrentPercentage)) (<= (LocalVariables|GetCurrentPercentage) (* (+ _index 1) (/ 100 _returnvalue))))
              ;[1 1 1] Win in range
              (Development|PrintString (Utilities|String|Append "Returned index:" (Utilities|String|ToString(Integer) _index) "/" (Utilities|String|Append (Utilities|String|ToString(Integer) (* _index (/ 100 _returnvalue))) "-" (Utilities|String|ToString(Integer) (* (+ _index 1) (/ 100 _returnvalue))) "+" (Utilities|String|ToString(Boolean) (and (< (* _index (/ 100 _returnvalue)) (LocalVariables|GetCurrentPercentage)) (<= (LocalVariables|GetCurrentPercentage) (* (+ _index 1) (/ 100 _returnvalue))))))) true true "(R=0.000000,G=0.660000,B=1.000000,A=1.000000)" 2e+01)
              (return (Utilities|Array|Get(acopy) (LocalVariables|GetFilteredArray) _index) true)
              (elif (== (LocalVariables|GetCurrentPercentage) (* (+ _index 1) (/ 100 _returnvalue)))
                ;[1 1 1] Win celing ==
                (Development|PrintString (Utilities|String|Append "Returned index:" (Utilities|String|ToString(Integer) _index) "/" (Utilities|String|Append (Utilities|String|ToString(Integer) (* _index (/ 100 _returnvalue))) "-" (Utilities|String|ToString(Integer) (* (+ _index 1) (/ 100 _returnvalue))) "+" (Utilities|String|ToString(Boolean) (== (LocalVariables|GetCurrentPercentage) (* (+ _index 1) (/ 100 _returnvalue)))))) true true "(R=0.000000,G=0.660000,B=1.000000,A=1.000000)" 2e+01)
                (return (Utilities|Array|Get(acopy) (LocalVariables|GetFilteredArray) _index) true)
                (else
                  ;[1 1 1] No meet, resume
                  (Development|PrintString (Utilities|String|Append (Utilities|String|ToString(Integer) (* _index (/ 100 _returnvalue))) "-" (Utilities|String|ToString(Integer) (* (+ _index 1) (/ 100 _returnvalue))) "+" (Utilities|String|ToString(Boolean) (and (< (* _index (/ 100 _returnvalue)) (LocalVariables|GetCurrentPercentage)) (<= (LocalVariables|GetCurrentPercentage) (* (+ _index 1) (/ 100 _returnvalue)))))) true true "(R=0.000000,G=0.660000,B=1.000000,A=1.000000)" 8e+01)))))
          ;[1 1 1] Loop fail
          (Development|PrintString "For loop completeed with no success in loop body")
          (return 0 false))))))