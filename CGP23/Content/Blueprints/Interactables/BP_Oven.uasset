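; Interactable oven that cooks held food items and pays out through a quick-time event.
; Interaction attempts removal, then looks up the held item's linked oven data row and, if idle, starts cooking and consumes it.
; A one-shot timer ends the cook while a looping timer tracks progress.
; Finished food triggers the QTE component, with spawn events producing the output or burned food plus happy or angry sheep effects.
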(event Custom|FinishCook
  (Utilities|Time|ClearandInvalidateTimerbyHandle (stale Custom|BeginCook _returnvalue_2))
  (Variables|Default|SetisCooking false))

(event Custom|BeginCook
  (bind _returnvalue (Utilities|Time|SetTimerbyEvent (delegate Custom|FinishCook) (.CookTime (Utilities|Struct|BreaksFood (Variables|Default|GetCurrentCook)))))
  (bind _returnvalue_2 (Utilities|Time|SetTimerbyEvent (delegate Custom|CookRapidEvent) 0.025 true)))

(event Custom|CookRapidEvent
  (Variables|Default|SetCookPercentage (/ (Class|KismetSystemLibrary|GetTimerElapsedTimeHandle (stale Custom|BeginCook _returnvalue)) (.CookTime (Utilities|Struct|BreaksFood (Variables|Default|GetCurrentCook))))))

(event Custom|SpawnItem
  (bind _returnvalue (Game|GetPlayerCharacter 0))
  (bind _returnvalue_2 (Transformation|GetActorLocation _returnvalue))
  (Game|SpawnActorfromClass "/Game/Blueprints/Inventory/BP_BaseItem.BP_BaseItem_C" (Math|Transform|MakeTransform _returnvalue_2 "0, 0, 0" "1.000000,1.000000,1.000000") "Undefined" "MultiplyWithRoot" 0 (.outputitem (Variables|Default|GetCurrentCook)) 0)
  (Niagara|SpawnSystematLocation "/Game/VFX/EmotionSprites/NS_SheepHappy.NS_SheepHappy" (+ _returnvalue_2 "-150.000000,0.000000,150.000000"))
  (Variables|Default|SetCurrentCook "")
  (Variables|Default|SetCookPercentage 0.0))

(event Custom|SpawnBurned
  (bind _returnvalue (Game|GetPlayerCharacter 0))
  (bind _returnvalue_2 (Transformation|GetActorLocation _returnvalue))
  (Game|SpawnActorfromClass "/Game/Blueprints/Inventory/BP_BaseItem.BP_BaseItem_C" (Math|Transform|MakeTransform _returnvalue_2 "0, 0, 0" "1.000000,1.000000,1.000000") "Undefined" "MultiplyWithRoot" 0 (Utilities|Struct|MakeDataTableRowHandle "/Game/Static_Data/Item/DT_Items.DT_Items" "BurnedFood") 0)
  (Niagara|SpawnSystematLocation "/Game/VFX/EmotionSprites/NS_SheepAngry.NS_SheepAngry" (+ _returnvalue_2 "-150.000000,0.000000,150.000000"))
  (Variables|Default|SetCurrentCook "")
  (Variables|Default|SetCookPercentage 0.0))

(event EventBeginPlay
  (bind _bpc_qtelogic (Variables|Default|GetBPC_QTELogic))
  (|CallParentFunction)
  (EventDispatchers|BindEventtoQTESuccess _bpc_qtelogic (EventDispatchers|CreateEvent :!event Custom|SpawnItem))
  (EventDispatchers|BindEventtoQTEFail _bpc_qtelogic (EventDispatchers|CreateEvent :!event Custom|SpawnBurned)))

(fn ConstructionScript
  (|CallParentFunction))

(fn AttemptCook
  (params (Food :type S%20Food%20Structure))
  (if (Variables|Default|GetisCooking)
    (return false)
    (else
      (Variables|Default|SetCurrentCook Food)
      (Variables|Default|SetisCooking true)
      (CallFunction|BeginCook)
      (return true))))

(fn AttemptRemoval
  (if (and (>= (Variables|Default|GetCookPercentage) 0.99) (not (Variables|Default|GetisCooking)))
    (Default|StartQTE (Variables|Default|GetBPC_QTELogic) 0.4 3.0 0.1)
    (else
      (Development|PrintString "Not Ready For Harvest"))))

(fn InteractionwithHeldItem
  (params (ItemInHand :type S%20Item%20Structure))
  (bind (_itemname _texture _amount_shouldbe1 _isstackable _maxstack _mesh _linkedgrowdata _linkedovendata) (Utilities|Struct|BreaksItem ItemInHand))
  (bind (_datatable _rowname) (Utilities|Struct|BreakDataTableRowHandle _linkedovendata))
  (|CallParentFunction ItemInHand)
  (CallFunction|AttemptRemoval)
  (if (Utilities|Enum|Equal(Enum) _itemname (Utilities|Text|MakeLiteralText "AIR"))
    (Development|PrintString "Empty Hand")
    (elif (== _rowname "EMPTY")
      (Development|PrintString "NO COOKABLE ASSOCIATED")
      (else
        (bind _returnvalue (Utilities|GetDataTableRow _datatable _rowname)
          (:then
            (bind _success (CallFunction|AttemptCook _returnvalue))
            (if _success
              (Default|RemoveItem (.OwningInventory-IGNORE (Utilities|Struct|BreaksItem ItemInHand)) ItemInHand))))))))