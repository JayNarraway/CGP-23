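; BP_Water is an interactable water body that runs a fishing minigame when used with a FishingRod.
; The first interaction locks player movement, spawns a lure, then after a random wait opens a three-second bite window.
; Interacting again ends fishing; a catch takes its quality from the bite timer, read after a delay.
; RawFish item data comes from a temporary far-off BP_BaseItem, destroyed once added to inventory.
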(event Custom|FindTime)

(event Custom|Begin
  (if (Variables|Default|GetRodFound)
    (bind _as_player (Utilities|Casting|CastTo_PLAYER (Game|GetPlayerCharacter 0)))
    (if (Variables|Default|GetIs%20Fishing)
      (Variables|Default|SetSend%20to%20Anim false)
      (if (Variables|Default|GetFish%20Ready)
        (Utilities|FlowControl|Delay 4.0)
        (Development|PrintString (Utilities|String|ToString(Float) (- 1e+02 (* (/ (Class|KismetSystemLibrary|GetTimerElapsedTimeHandle (stale _returnvalue_3)) 3.0) 1e+02))))
        (Development|PrintString (Utilities|String|ToString(Float) (Class|KismetSystemLibrary|GetTimerElapsedTimeHandle (stale _returnvalue_3))))
        (if (< (Class|KismetSystemLibrary|GetTimerElapsedTimeHandle (stale _returnvalue_3)) 3.0)
          (if (Variables|Default|GetCan%20Spawn)
            ;[1 1 1] This entire section is incredibly stupid, if anyone would like to try and improve it by all means but it works and fuck trying to optimise it, asset duping is a bitch
            (bind _returnvalue (Game|SpawnActorfromClass "/Game/Blueprints/Inventory/BP_BaseItem.BP_BaseItem_C" (Math|Transform|MakeTransform "99999999.000000,0.000000,0.000000" "0, 0, 0" "1.000000,1.000000,1.000000") "Undefined" "MultiplyWithRoot" 0 (Utilities|Struct|MakeDataTableRowHandle "/Game/Static_Data/Item/DT_Items.DT_Items" "RawFish") 0))
            (Variables|Default|SetCan%20Spawn false)
            (bind _structout (Utilities|Struct|SetmembersinsItem (Variables|/Game/Blueprints/Inventory/BP_BaseItem.BP_BaseItem_C|GetItemData _returnvalue) (Math|Float|Truncate (- 1e+02 (* (/ (Class|KismetSystemLibrary|GetTimerElapsedTimeHandle (stale _returnvalue_3)) 3.0) 1e+02)))))
            (Default|AddItemtoInventory (Variables|/Game/Player/_PLAYER._PLAYER_C|GetBPC_Inventory _as_player) _structout)
            (Development|PrintString (Utilities|String|ToString(Integer) (.ItemQuality-IGNORE (Utilities|Struct|BreaksItem _structout))) true true "(R=0.120151,G=0.307292,B=0.105708,A=1.000000)")
            (Actor|DestroyActor _returnvalue))
          (Variables|Default|SetFailed true :!label _label)
          (Variables|Default|SetIs%20Fishing false)
          (Variables|Default|SetReady%20Time -1e+02)
          (Variables|Default|SetFish%20Ready false)
          (Pawn|Components|CharacterMovement|SetMovementMode (Variables|/Script/Engine.Character|GetCharacterMovement _as_player) "MOVE_Walking" 0)
          (Actor|DestroyActor (stale _returnvalue_2))
          (Variables|Default|SetFish%20Wait%20Time -9999.0))
        (else
          (Development|PrintString "FISHING FAILED")
          (goto _label)))
      (else
        (Variables|Default|SetSend%20to%20Anim true)
        (Pawn|Components|CharacterMovement|DisableMovement (Variables|/Script/Engine.Character|GetCharacterMovement _as_player))
        (Utilities|FlowControl|Delay 4.5)
        (bind _returnvalue_2 (Game|SpawnActorfromClass "/Game/Blueprints/Interactables/Fishing_Visuals/BP_FishingLure.BP_FishingLure_C" (Math|Transform|MakeTransform (+ (Transformation|GetActorForwardVector _as_player) (Transformation|GetActorLocation _as_player)) (Math|Rotator|FindLookatRotation (Transformation|GetActorLocation _as_player) (Transformation|GetWorldLocation (Variables|Default|GetDefaultSceneRoot))) "1.000000,1.000000,1.000000") "Undefined" "MultiplyWithRoot" 0 0))
        (Development|PrintString "FISH START")
        (Variables|Default|SetFailed false)
        (Variables|Default|SetIs%20Fishing true)
        (bind _output_get (Variables|Default|SetFish%20Wait%20Time (Math|Random|RandomFloatinRange 2.0 3.0)))
        (Pawn|Components|CharacterMovement|DisableMovement (Variables|/Script/Engine.Character|GetCharacterMovement _as_player))
        (Utilities|FlowControl|Delay _output_get)
        (if (not (Variables|Default|GetFailed))
          (Variables|Default|SetReady%20Time (stale EventTick DeltaSeconds))
          (Development|PrintString "FISH READY")
          (bind _returnvalue_3 (Utilities|Time|SetTimerbyEvent (delegate Custom|FindTime) 3.0))
          (Variables|Default|SetCan%20Spawn true)
          (Variables|Default|SetFish%20Ready true)
          (bind _returnvalue_4 (Actor|GetActorOfClass "/Game/Blueprints/Interactables/Fishing_Visuals/BP_FishingLure.BP_FishingLure_C"))
          (if (not (Variables|Default|GetFailed))
            (Default|ReceiveFishReady _returnvalue_4)
            (Utilities|FlowControl|Delay 3.0)
            (if (not (Variables|Default|GetFailed))
              (Default|ReceiveFishGone _returnvalue_4)
              (Variables|Default|SetFish%20Ready false)
              (Development|PrintString "FISH MISSED"))))))))

(event EventTick
  (params (DeltaSeconds :type Float%20%28single-precision%29)))

(fn ConstructionScript
  (|CallParentFunction))

(fn InteractionwithHeldItem
  (params (ItemInHand :type S%20Item%20Structure))
  (if (Utilities|Enum|Equal(Enum) (.ItemName (Utilities|Struct|BreaksItem ItemInHand)) (Utilities|Text|MakeLiteralText "FishingRod"))
    (Variables|Default|SetRodFound true)
    (else
      (Variables|Default|SetRodFound false)))
  (CallFunction|Begin))