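; BP_Bed is an interactable bed that runs a timed sequence on the player.
; Interact finds the player actor, disables its input and teleports it to the first arrow component while the TOAnim flag is raised.
; After fixed delays it clears the flag, moves the player to a second arrow, then restores input and places it at a final arrow transform.
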(event EventBeginPlay)

(event Collision|EventActorBeginOverlap
  (params (OtherActor :type Actor%20Object%20Reference)))

(event EventTick
  (params (DeltaSeconds :type Float%20%28single-precision%29)))

(event EventInteract
  (params (HitComponent :type Primitive%20Component%20Object%20Reference) (ItemInHand :type S%20Item%20Structure))
  (bind _arroww (Variables|Default|GetArroww))
  (bind _arroww2 (Variables|Default|GetArroww2))
  (bind _returnvalue (Transformation|GetWorldTransform _arroww2))
  (bind _returnvalue_2 (Transformation|GetWorldTransform _arroww))
  (bind _returnvalue_3 (Actor|GetActorOfClass "/Game/Player/_PLAYER._PLAYER_C"))
  (bind _output_get (Variables|Default|SetAs%20PLAYER _returnvalue_3))
  (Input|DisableInput _output_get 0)
  (Transformation|SetActorLocationAndRotation _output_get (.location _returnvalue_2) (.rotation _returnvalue_2) false true)
  (Variables|Default|SetTO%20anim true)
  (Utilities|FlowControl|Delay 3.17)
  (Variables|Default|SetTO%20anim false)
  (Transformation|SetActorLocationAndRotation (Variables|Default|GetAs%20PLAYER) (.location _returnvalue) (.rotation _returnvalue) false true)
  (Utilities|FlowControl|Delay 4.8)
  (Input|EnableInput (Variables|Default|GetAs%20PLAYER) 0)
  (Transformation|SetActorTransform (Variables|Default|GetAs%20PLAYER) (Transformation|GetWorldTransform (Variables|Default|GetArrowwPURE)) false true))

(fn ConstructionScript
  (|CallParentFunction))