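; BP_InteractableMaster is a base interactable that shows its name on the player's HUD and accepts an interaction with a held item.
; Collision overlap begin caches player 0's _PLAYER and displays ObjectName, and overlap end hides the prompt, with neither event checking which actor overlapped.
; The Interact event forwards ItemInHand to InteractionWithHeldItem, which is an empty function here.
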(event OnComponentBeginOverlap(Collision)
  (params (OverlappedComponent :type Primitive%20Component%20Object%20Reference) (OtherActor :type Actor%20Object%20Reference) (OtherComp :type Primitive%20Component%20Object%20Reference) (OtherBodyIndex :type Integer) (bFromSweep :type Boolean) (SweepResult :type Hit%20Result%20Structure%20%28by%20ref%29))
  (bind _as_player (Utilities|Casting|CastTo_PLAYER (Game|GetPlayerCharacter 0)))
  (bind _output_get (Variables|Default|SetAs%20PLAYER _as_player))
  (Default|DisplayInteraction (Variables|/Game/Player/_PLAYER._PLAYER_C|GetAsHUD _output_get) (Variables|Default|GetObjectName) false))

(event OnComponentEndOverlap(Collision)
  (params (OverlappedComponent :type Primitive%20Component%20Object%20Reference) (OtherActor :type Actor%20Object%20Reference) (OtherComp :type Primitive%20Component%20Object%20Reference) (OtherBodyIndex :type Integer))
  (bind _as_player (Variables|Default|GetAs%20PLAYER)
    (:then
      (Default|DisplayInteraction (Variables|/Game/Player/_PLAYER._PLAYER_C|GetAsHUD _as_player) "" true))
    (:else)))

(event EventInteract
  (params (HitComponent :type Primitive%20Component%20Object%20Reference) (ItemInHand :type S%20Item%20Structure))
  (CallFunction|InteractionwithHeldItem ItemInHand))

(fn ConstructionScript)

(fn InteractionwithHeldItem
  (params (ItemInHand :type S%20Item%20Structure)))