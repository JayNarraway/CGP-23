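; BP_BaseItem is a pickup actor that adds itself to the inventory of an actor overlapping its sphere.
; The construction script looks up the Type data table row, stores it as ItemData and sets the mesh from it.
; On overlap it passes ItemData to BPC_Inventory and destroys itself if the add succeeds.
; Any BPC_InventoryQuestChecker on that actor receives the row name with quantity one, even if the add fails.
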(event OnComponentBeginOverlap(Sphere)
  (params (OverlappedComponent :type Primitive%20Component%20Object%20Reference) (OtherActor :type Actor%20Object%20Reference) (OtherComp :type Primitive%20Component%20Object%20Reference) (OtherBodyIndex :type Integer) (bFromSweep :type Boolean) (SweepResult :type Hit%20Result%20Structure%20%28by%20ref%29))
  (bind _returnvalue (Actor|GetComponentbyClass OtherActor "/Game/Blueprints/Inventory/BPC_Inventory.BPC_Inventory_C"))
  (bind _returnvalue_2 (Actor|GetComponentbyClass OtherActor "/Game/Tech/BuildingNQuests/Blueprints/QuestSys/BPC_InventoryQuestChecker.BPC_InventoryQuestChecker_C"))
  (if (Utilities|IsValid _returnvalue)
    (bind _success (Default|AddItemtoInventory _returnvalue (Variables|Default|GetItemData)))
    ;[0 1 0.9527] Inventory Quest Checker
    (Utilities|IsValid _returnvalue_2
      (:Is%20Valid
        (Default|AddtoInventory _returnvalue_2 (.RowName (Utilities|Struct|BreakDataTableRowHandle (Variables|Default|GetType))) 1))
      (:Is%20Not%20Valid
        _))
    (if _success
      (Actor|DestroyActor))))

(fn ConstructionScript
  (bind _type (Variables|Default|GetType))
  (bind _returnvalue (Utilities|GetDataTableRow (.datatable _type) (.rowname _type))
    (:then
      (bind _output_get (Variables|Default|SetItemData _returnvalue))
      (Components|StaticMesh|SetStaticMesh (Variables|Default|GetItemMesh) (.Mesh (Utilities|Struct|BreaksItem _output_get))))))