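; Inventory component that stores item structs in a size-capped array and calls InventoryUpdated after successful adds and on removals.
; Adding tops up the first same-named stack one unit at a time, then puts any remainder in a new slot stamped with owning inventory and slot index.
; CheckForItem looks items up by name, while RemoveItem matches the whole struct to decrement its amount or drop the entry.
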(fn AddItemtoInventory
  (params (inItemData :type S%20Item%20Structure%20%28by%20ref%29))
  (bind _success (CallFunction|TryAddtoStack inItemData))
  (if _success
    (Default|CallInventoryUpdated))
  (return _success))

(fn TryAddtoStack
  (params (ItemData :type S%20Item%20Structure%20%28by%20ref%29))
  (bind (_itemname _texture _amount) (Utilities|Struct|BreaksItem ItemData))
  (bind _returnvalue (> _amount 0))
  (for (_array_element _array_index) (Variables|Default|GetInventory) ; loop through all stacks
    (if (Utilities|Enum|Equal(Enum) _itemname (.ItemName (Utilities|Struct|BreaksItem _array_element))) ; if one is found which items have the same name as incoming
      (while (and _returnvalue (< (.Amount (Utilities|Struct|BreaksItem _array_element)) (.MaxStack (Utilities|Struct|BreaksItem _array_element)))) ; begin transfer of stack
        (Utilities|Struct|SetmembersinsItem ItemData (- (.Amount (Utilities|Struct|BreaksItem ItemData)) 1))
        (bind _structout (Utilities|Struct|SetmembersinsItem _array_element (+ (.Amount (Utilities|Struct|BreaksItem _array_element)) 1)))
        (Utilities|Array|SetArrayElem (Variables|Default|GetInventory) _array_index _structout))
      (if _returnvalue ; if there is any left
        (bind _success (CallFunction|AddNewStack ItemData))
        (return _success)
        (else
          (return true)))))
  (if _returnvalue ; if there is any left
    (bind _success_2 (CallFunction|AddNewStack ItemData))
    (return _success_2)
    (else
      (return true))))

(fn AddNewStack
  (params (ItemData :type S%20Item%20Structure))
  (bind (_itemname _texture _amount _isstackable _maxstack _mesh _linkedgrowable _linkedcook) (Utilities|Struct|BreaksItem ItemData))
  (bind _inventory (Variables|Default|GetInventory))
  (if (< (Utilities|Array|Length _inventory) (Variables|Default|GetMaxInventorySize))
    (bind _returnvalue (Utilities|Array|Add _inventory ItemData))
    (Utilities|Array|SetArrayElem _inventory _returnvalue (Utilities|Struct|MakesItem _itemname _texture _amount _isstackable _maxstack _mesh _linkedgrowable _linkedcook self _returnvalue))
    (return true)
    (else
      (return false))))

(fn CheckforItem
  (params (ItemName :type Text))
  (LocalVariables|SetitemFound false)
  (LocalVariables|SetLocatedItem "")
  (bind _array_element (Utilities|Array|ForEachLoopwithBreak (Variables|Default|GetInventory))
    (:LoopBody
      (if (Utilities|Enum|Equal(Enum) ItemName (.ItemName (Utilities|Struct|BreaksItem _array_element)))
        (LocalVariables|SetitemFound true)
        (LocalVariables|SetLocatedItem _array_element)))
    (:Completed
      (return (LocalVariables|GetitemFound) (LocalVariables|GetLocatedItem)))))

(fn RemoveItem
  (params (ItemData :type S%20Item%20Structure))
  (bind (_itemname _texture _amount _isstackable _maxstack _mesh _linkedgrowable _linkedcook _owninginventory_ignore _slotnumber_ignore) (Utilities|Struct|BreaksItem ItemData))
  (bind _inventory (Variables|Default|GetInventory))
  (bind _returnvalue (Utilities|Array|FindItem _inventory ItemData))
  (if (> (.Amount (Utilities|Struct|BreaksItem ItemData)) 1)
    (if (!= _returnvalue -1)
      (Utilities|Array|SetArrayElem _inventory _returnvalue (Utilities|Struct|MakesItem _itemname _texture (- _amount 1) _isstackable _maxstack _mesh _linkedgrowable _linkedcook _owninginventory_ignore _slotnumber_ignore))
      (Default|CallInventoryUpdated)
      (return true)
      (else
        (return false)))
    (else
      (Utilities|Array|RemoveItem (Variables|Default|GetInventory) ItemData)
      (Default|CallInventoryUpdated)
      (return true))))