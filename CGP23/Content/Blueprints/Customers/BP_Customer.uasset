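; BP_Customer is a customer actor that shows a food order on a billboard and accepts the matching held item.
; The first interaction reveals the preset DesiredFood, and later ones compare item names, printing the result.
; A match removes the item, hides the customer, notifies the manager and pays MaxValue through the player's BPC_Currency.
; A positive payout spawns Niagara coins at a hardcoded location, with the count set from MaxValue.
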(event Custom|Select%20food
  (bind _foodbillboard (Variables|Default|GetFoodBillboard))
  ;[0.901 0.5591 0.3091] Select food
  (Rendering|Components|Sprite|SetSprite _foodbillboard (.Texture (Utilities|Struct|BreaksItem (Variables|Default|GetDesired%20Food))))
  (Components|Activation|SetActive _foodbillboard true false)
  (Variables|Default|SetGivenOrder true))

(event EventBeginPlay
  (Components|Activation|SetActive (Variables|Default|GetFoodBillboard) false false))

(event EventInteractionwithHeldItem
  (params (ItemInHand :type S%20Item%20Structure))
  (bind (_itemname _texture _amount_shouldbe1 _isstackable _maxstack _mesh _linkedgrowdata _linkedovendata _linkedpotdata _linkedchopdata _itemquality_ignore _owninginventory_ignore) (Utilities|Struct|BreaksItem ItemInHand))
  (bind _maxvalue (Variables|Default|GetMaxValue))
  (bind _foodbillboard (Variables|Default|GetFoodBillboard))
  ;[0 1 0.0264] Interaction
  (if (Variables|Default|GetGivenOrder)
    (if (Utilities|Enum|Equal(Enum) _itemname (.ItemName (Utilities|Struct|BreaksItem (Variables|Default|GetDesired%20Food))))
      (Default|RemoveItem _owninginventory_ignore ItemInHand)
      (Development|PrintString "CORRECT  Item")
      (Rendering|Components|Sprite|SetSprite _foodbillboard 0)
      (Components|Activation|SetActive _foodbillboard false false)
      (Variables|Default|SetGivenOrder false)
      (Rendering|SetActorHiddenInGame true)
      (Components|Activation|SetActive (Variables|Default|GetDefaultSceneRoot) false false)
      (Default|OrderCompleat (Variables|Default|GetManger))
      (Default|ChangeCurrency (Actor|GetComponentbyClass (Game|GetPlayerCharacter 0) "/Game/Tech/Currency/BPC_Currency.BPC_Currency_C") _maxvalue)
      ;[1 1 1] VFX
      (if (> _maxvalue 0)
        (bind _output_get (Variables|Default|SetCoinLoc "1400.000000,99.999991,350.000000"))
        (bind _returnvalue (Niagara|SpawnSystematLocation "/Game/VFX/NS_Coins.NS_Coins" _output_get))
        (Class|NiagaraComponent|SetVariableInt _returnvalue "COINCOUNT" _maxvalue)
        (Niagara|SpawnSystematLocation 0 "0, 0, 0"))
      (else
        (Development|PrintString "Incorrect Item")))
    (else
      (CallFunction|SelectFood))))

(fn ConstructionScript
  (|CallParentFunction))