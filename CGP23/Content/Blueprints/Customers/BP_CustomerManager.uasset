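; Customer manager actor that runs a day's food orders through a reused pool of three BP_Customer actors, spawned hidden and inactive on BeginPlay.
; SetUpDay draws random orders from the selected menu DataTable, and OverrideItem can replace specific entries.
; NewCustomer activates idle customers with queued orders, and OrderCompleat refills them after a delay or calls the empty End hook when all are done.
; BeginPlay currently starts a hardcoded test day.
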(event Custom|Set%20Up%20Day
  (params (NumOfOrders :type Integer) (MenuOfDay :type ENM_Menu%20Enum :default "NewEnumerator0"))
  ;[0 0.853 1] Creates a list of orders. make sure to call this before anything esles
  (bind _output_get (Variables|Default|SetMenuENM MenuOfDay))
  (Variables|Default|SetNumOfOrders NumOfOrders)
  (bind _menudatatable (CallFunction|SelectMenu _output_get))
  (bind _outrownames (DataTable|GetDataTableRowNames _menudatatable))
  (for _index (range 0 (Variables|Default|GetNumOfOrders))
    (bind _returnvalue (Utilities|GetDataTableRow (Variables|Default|GetMenuDT) (.OutItem (Utilities|Array|Random _outrownames)))
      (:then
        (Utilities|Array|Add (Variables|Default|GetOrders) _returnvalue)))))

(event Custom|Override%20Item
  (params (Position :type Integer) (Item :type S%20Menu%20Structure))
  (bind _itemref (Utilities|Struct|BreakSMenu Item))
  (bind (_datatable _rowname) (Utilities|Struct|BreakDataTableRowHandle _itemref))
  ;[1 0 0.8743] Override an item in the order list to have a specfic item. Call this after Set Up Day
  (if (> Position (Utilities|Array|Length (Variables|Default|GetOrders)))
    (bind _returnvalue (Utilities|GetDataTableRow _datatable _rowname)
      (:then
        (Utilities|String|LogString (Utilities|String|Append "Unable to add item: \"" (Utilities|String|ToString(Text) (.ItemName (Utilities|Struct|BreaksItem _returnvalue))) "\". Out of range of array"))))
    (else
      (Utilities|Array|SetArrayElem (Variables|Default|GetOrders) Position Item))))

(event Custom|New%20Customer
  (bind _orders (Variables|Default|GetOrders))
  (bind _orders_2 (Variables|Default|GetOrders))
  (bind _output (Utilities|Array|Get(acopy) _orders))
  (bind (_itemref _value) (Utilities|Struct|BreakSMenu _output))
  (bind (_datatable _rowname) (Utilities|Struct|BreakDataTableRowHandle _itemref))
  ;[0.3075 1 0] Assign Orders to customers
  (if (not (Utilities|Array|IsEmpty (Variables|Default|GetOrders)))
    (bind _array_element (Utilities|Array|ForEachLoopwithBreak (Variables|Default|GetCustomers) :!label _label)
      (:LoopBody
        (if (not (Components|Activation|IsActive (Variables|/Script/Engine.Actor|GetRootComponent _array_element)))
          (Components|Activation|SetActive (Variables|/Script/Engine.Actor|GetRootComponent _array_element) true false)
          (Rendering|SetActorHiddenInGame _array_element false)
          (Variables|/Game/Blueprints/Customers/BP_Customer.BP_Customer_C|SetMaxValue _array_element _value)
          (bind _returnvalue (Utilities|GetDataTableRow _datatable _rowname)
            (:then
              (Variables|/Game/Blueprints/Customers/BP_Customer.BP_Customer_C|SetDesired%20Food _array_element _returnvalue)
              (Default|SelectFood _array_element)
              (Utilities|Array|RemoveIndex _orders_2)
              (if (Utilities|Array|IsEmpty _orders_2)
                (goto _label Break)))))))))

(event Custom|End
  ;[0.1298 0 1] Triggers for things to happen when finished with customers
)

(event Custom|Order%20Compleat
  ;[1 0.3929 0] Actions for after an order has been handed in
  (if (Utilities|Array|IsEmpty (Variables|Default|GetOrders))
    (bind _output_get (Variables|Default|SetContinue false))
    (bind _array_element (Utilities|Array|ForEachLoopwithBreak (Variables|Default|GetCustomers) :!label _label)
      (:LoopBody
        (if (Components|Activation|IsActive (Variables|/Game/Blueprints/Interactables/BP_InteractableMaster.BP_InteractableMaster_C|GetDefaultSceneRoot _array_element))
          (Variables|Default|SetContinue true)
          (goto _label Break)))
      (:Completed
        (if _output_get
          (Utilities|FlowControl|Delay 5.0 :!label _label_2)
          (CallFunction|NewCustomer)
          (else
            (CallFunction|End)))))
    (else
      (goto _label_2))))

(event Collision|EventActorBeginOverlap
  (params (OtherActor :type Actor%20Object%20Reference)))

(event EventTick
  (params (DeltaSeconds :type Float%20%28single-precision%29)))

(event EventBeginPlay
  ;[0 0.1337 1] Setup customers
  (for _index (range 0 2)
    (bind _returnvalue (Game|SpawnActorfromClass "/Game/Blueprints/Customers/BP_Customer.BP_Customer_C" (Math|Transform|MakeTransform (+ (Utilities|Array|Get(acopy) (Variables|Default|GetSpawn%20Location) _index) (.location (Transformation|GetActorTransform))) "0, 0, 0" "1.000000,1.000000,1.000000") "Undefined" "MultiplyWithRoot" 0 0))
    (Rendering|SetActorHiddenInGame _returnvalue true)
    (Components|Activation|SetActive (Variables|/Script/Engine.Actor|GetRootComponent _returnvalue) false false)
    (Variables|/Game/Blueprints/Customers/BP_Customer.BP_Customer_C|SetManger _returnvalue self)
    (Utilities|Array|Add (Variables|Default|GetCustomers) _returnvalue))
  ;;[1 0 0] remove this once you have a trigger for new day
  (CallFunction|SetUpDay 2 "NewEnumerator0")
  (CallFunction|NewCustomer))

(fn ConstructionScript)

(fn SelectMenu
  (params (MenuToPickFrom :type Byte))
  ;[1 0 0] When adding new menus add here
  (switch Utilities|FlowControl|Switch|Switchon MenuToPickFrom
    (:NewEnumerator0
      (Variables|Default|SetMenuDT "/Game/Static_Data/SMenu/DT_Menu0.DT_Menu0"))
    (:NewEnumerator1
      (Variables|Default|SetMenuDT "/Game/Static_Data/SMenu/DT_Menu1.DT_Menu1")))
  (return (Variables|Default|GetMenuDT)))