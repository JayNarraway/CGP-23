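; Animation notify that spawns walking rubble VFX at the player's left foot.
; It spawns NS_WalkingRubble at the leg_toe_l socket, then feeds its VELOCITY parameter the character's last movement velocity, scaled down and reversed.
; Socket and velocity come from player character 0, not the notifying MeshComp.
; A leftover FlipFlop node is never executed.
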(fn ReceivedNotify
  (params (MeshComp :type Skeletal%20Mesh%20Component%20Object%20Reference) (Animation :type Anim%20Sequence%20Base%20Object%20Reference) (EventReference :type Anim%20Notify%20Event%20Reference%20Structure%20%28by%20ref%29))
  (bind _returnvalue (Game|GetPlayerCharacter 0))
  (bind _returnvalue_2 (Niagara|SpawnSystematLocation "/Game/VFX/NS_WalkingRubble.NS_WalkingRubble" (.location (Transformation|GetSocketTransform (Variables|/Script/Engine.Character|GetMesh _returnvalue) "leg_toe_l" "RTS_World"))))
  (Niagara|SetNiagaraVariable(Vector3) _returnvalue_2 "VELOCITY" (* (/ (Pawn|Components|CharacterMovement|GetLastUpdateVelocity (Variables|/Script/Engine.Character|GetCharacterMovement _returnvalue)) "100.000000,100.000000,100.000000") "-1.000000,-1.000000,-1.000000"))
  (return false))